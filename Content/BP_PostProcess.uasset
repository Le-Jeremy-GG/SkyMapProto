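; BP_PostProcess is an actor that crossfades between day and night post-process looks.
; The PostProcessSetBlend event passes an alpha to SetBlendDay, which gives PPDay that blend weight and PPNight the inverse.
; Both SetDay branches call SetBlendDay and differ only in debug print color, leaving the mirrored SetBlendNight unused.
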(event `self.ReceiveTick`
  (params (DeltaSeconds :type "Float (single-precision)")))

(event `/Game/Main/Constellations/Interfaces/BPI_GMConstell.PostProcessSetBlend`
  (params (NewAlpha :type "Float (single-precision)") (SetDay :type Boolean))
  (bind _returnvalue (`KismetStringLibrary.Conv_DoubleToString` NewAlpha))
  (if SetDay
    (`self.SetBlendDay` NewAlpha)
    (`KismetSystemLibrary.PrintString` _returnvalue true true (struct :`R` 1.0 :`G` 0.063079 :`B` 0.192847 :`A` 1.0))
    (else
      (`self.SetBlendDay` NewAlpha)
      (`KismetSystemLibrary.PrintString` _returnvalue true true (struct :`G` 0.722498 :`B` 1.0 :`A` 1.0)))))

(fn `SetBlendDay`
  (params (Alpha :type "Float (double-precision)"))
  ;[1 1 1] Set le blend quand on passe du jour a la nuit
  (set `PostProcessComponent.BlendWeight` Alpha (`self.PPDay`))
  (set `PostProcessComponent.BlendWeight` (- 1.0 Alpha) (`self.PPNight`)))

(fn `SetBlendNight`
  (params (Alpha :type "Float (double-precision)"))
  ;[1 1 1] Set le blend quand on passe de la nuit au jour
  (set `PostProcessComponent.BlendWeight` Alpha (`self.PPNight`))
  (set `PostProcessComponent.BlendWeight` (- 1.0 Alpha) (`self.PPDay`)))

(fn `UserConstructionScript`)