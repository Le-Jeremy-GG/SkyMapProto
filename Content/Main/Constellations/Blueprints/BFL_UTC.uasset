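; Blueprint function library that converts date-times between local time and UTC for a set of predefined Pacific time zones.
; GetPredefinedTimeZone maps the time zone enum to a row name in DT_TimeZones and returns that row's hour offset.
; LocalToUTC and UTCToLocal turn the offset into whole minutes, so fractional-hour zones work, then respectively remove or add it as a timespan.
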(fn `GetPredefinedTimeZone`
  (params (TimeZone :type "/Game/Main/Constellations/Datas/Enum_TimeZones Enum" :default "NewEnumerator0"))
  (returns (UTC :type "Float (double-precision)"))
  (bind _returnvalue (`|GetDataTableRow` "/Game/Main/Constellations/Datas/DT_TimeZones.DT_TimeZones" (select `/Game/Main/Constellations/Datas/Enum_TimeZones` TimeZone :`NewEnumerator0` "Tahiti" :`NewEnumerator1` "HivaOa" :`NewEnumerator2` "Hawai" :`NewEnumerator3` "NewZealand" :`NewEnumerator4` "RapaNui" :`NewEnumerator5` "NewCaledonia" :!type "Name"))
    (:`then`
      (return (`.TimeZone_11_9A354EC140D07EC0EE8FF9A3559B54BD` (break `/Game/Main/Constellations/Datas/Struct_TimeZones` _returnvalue))))))

(fn `LocalToUTC`
  (params (Local :type "DateTime Structure") (TimeZone :type "/Game/Main/Constellations/Datas/Enum_TimeZones Enum" :default "NewEnumerator0"))
  (returns (UTCTime :type "DateTime Structure"))
  (return (+ Local (`KismetMathLibrary.MakeTimespan` 0 0 (`KismetMathLibrary.FTrunc` (* (* (`self.GetPredefinedTimeZone` TimeZone) 60.0) -1.0))))))

(fn `UTCToLocal`
  (params (UTC :type "DateTime Structure") (TimeZone :type "/Game/Main/Constellations/Datas/Enum_TimeZones Enum" :default "NewEnumerator0"))
  (returns (Local :type "DateTime Structure"))
  (return (+ UTC (`KismetMathLibrary.MakeTimespan` 0 0 (`KismetMathLibrary.FTrunc` (* (`self.GetPredefinedTimeZone` TimeZone) 60.0))))))