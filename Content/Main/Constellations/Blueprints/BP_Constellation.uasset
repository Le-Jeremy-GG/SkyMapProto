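; Constellation actor that shows a star figure and its info widget in a VR sky scene.
; Given data and stars through ConstellSetConstellation, it spawns one BP_TieConstellation per star, passing each its target star and name.
; Opacity and refresh calls are relayed to every tie by message.
; At night, toggling opacity also shows or hides the WBP_Constellation world widget, placed along the camera's forward vector and rotated toward the pawn.
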(event `self.ReceiveBeginPlay`
  ;[1 1 1] Crée le widget et set l'opacité
  (`KismetSystemLibrary.Delay` 0.2)
  (`SceneComponent.SetVisibility` (`self.Widget`) false false)
  (bind _returnvalue (`|CreateWidget` "/Game/Main/Constellations/UserInterfaces/WBP_Constellation.WBP_Constellation_C" null (`self.ConstellationData`)))
  (`WidgetComponent.SetWidget` (`self.Widget`) _returnvalue)
  (`self.Constell_SetOpacity` false))

(event `self.Constell_SetOpacity`
  (params (Visible :type Boolean))
  ;[1 1 1] Set l'opacité de la constellation qd on interragit avec elle via le controleur
  (if (!= Visible (`self.bIsDisplayed`))
    (set `self.bIsDisplayed` Visible)
    (for _array_element (`self.TiesList`)
      (message `/Game/Main/Constellations/Interfaces/BPI_Stars.Constell_SetOpacity` _array_element (`self.bIsDisplayed`))
      (if (`/Game/Main/Constellations/Blueprints/BP_TimeManager.CheckIfNight` (struct))
        (`self.DisplayWidget` (`self.bIsDisplayed`))))))

(event `self.Constell_SetConstellation`
  (params (ConstellationData :type "/Game/Main/Constellations/Datas/Struct_Constellation Structure") (StarList :type "Array of Actor Object Reference (by ref)"))
  ;[1 1 1] Initialise la constellation depuis le Star Manager.
  ; Recupere les données et en spawn les liens et place le symbole illustrant la constellation
  (set `self.ConstellationData` ConstellationData)
  (set `self.StarsList` StarList)
  (`self.SpawnTies`))

(event `self.RefreshConstellations`
  ;[1 1 1] Envoie à chaque astre le signal pour se mettre a jour en fonction des etoiles. Puis calcule la position du symbole
  (for _array_element (`self.TiesList`)
    (message `/Game/Main/Constellations/Interfaces/BPI_Stars.RefreshConstellations` _array_element)))

(fn `DisplayWidget`
  (params (IsDisplayed :type Boolean))
  (bind _returnvalue (* (`SceneComponent.GetForwardVector` (`/Game/VirtualRealityBP/Blueprints/MotionControllerPawn.Camera` (cast `/Game/VirtualRealityBP/Blueprints/MotionControllerPawn` (`GameplayStatics.GetPlayerPawn` 0) :!pure true))) 1024.0))
  (if (and IsDisplayed true (`.bSuccess` (cast `/Game/VirtualRealityBP/Blueprints/MotionControllerPawn` (`GameplayStatics.GetPlayerPawn` 0) :!pure true)))
    ;[1 1 1] Si constellation est affichée, set la position du Widget à la vue du joueur et le rend visible
    (`SceneComponent.K2_SetWorldTransform` (`self.Widget`) (`KismetMathLibrary.MakeTransform` _returnvalue (`KismetMathLibrary.FindLookAtRotation` _returnvalue (`self.K2_GetActorLocation` (`GameplayStatics.GetPlayerPawn` 0)))) false false)
    (`SceneComponent.SetVisibility` (`self.Widget`) true false)
    (else
      ;[1 1 1] Sinon se contente de cacher le widget
      (`SceneComponent.SetVisibility` (`self.Widget`) false false)))
  (return))

(fn `SpawnTies`
  (locals (CurrentIndex :type Integer) (CurrentStar :type "Actor Object Reference"))
  (bind (_constellationdata_constellationname _constellationdata_description _constellationdata_degrees _constellationdata_starnamehr _constellationdata_startoaim _constellationdata_starnames) (break `/Game/Main/Constellations/Datas/Struct_Constellation` (`self.ConstellationData`)))
  (bind _value (`BlueprintMapLibrary.Map_Find` (`.StarToAim_50_F934EB5F498A5AD8A215C090CEF70F4C` (break `/Game/Main/Constellations/Datas/Struct_Constellation` (`self.ConstellationData`))) (`local.CurrentIndex`)))
  (for (_array_element _array_index) (`self.StarsList`)
    (set `local.CurrentStar` _array_element)
    (set `local.CurrentIndex` _array_index)
    ;[1 1 1] Spawn et liste le lien assigné à l'etoile actuellement loopée
    (bind _returnvalue (`|SpawnActorFromClass` "/Game/Main/Constellations/Blueprints/BP_TieConstellation.BP_TieConstellation_C" (`KismetMathLibrary.MakeTransform` (`self.K2_GetActorLocation` (`local.CurrentStar`))) "Undefined" "OverrideRootScale" null null))
    (`KismetArrayLibrary.Array_Add` (`self.TiesList`) _returnvalue)
    ;[1 1 1] Envoie tout ça au lien qui pourra ainsi gérer lui meme sa position et ses informations
    (message `/Game/Main/Constellations/Interfaces/BPI_Stars.TieConstell_SetAssignedStar` _returnvalue (`local.CurrentStar`) (select `bool` (!= _value -1) :`true` (`|GetArrayItem` (`self.StarsList`) _value)) self (`|GetArrayItem` _constellationdata_starnames (`local.CurrentIndex`)) (`local.CurrentIndex`)))
  (return))

(fn `UserConstructionScript`)