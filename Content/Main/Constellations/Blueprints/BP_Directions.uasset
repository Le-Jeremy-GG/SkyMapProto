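; Compass direction actor for the Constellations content, placing eight components for the cardinal and intercardinal points (N, S, E, W, NE, NW, SW, SE).
; The construction script calls SetDirectionDistance, which multiplies each component's world location by Distance to push it outward.
; Scaling uses world coordinates, so it is relative to the world origin rather than the actor's position.
; The event graph holds no runtime logic.
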(event `self.ReceiveTick`
  (params (DeltaSeconds :type "Float (single-precision)")))

(fn `SetDirectionDistance`
  (bind _s (`self.S`))
  (bind _e (`self.E`))
  (bind _w (`self.W`))
  (bind _ne (`self.NE`))
  (bind _nw (`self.NW`))
  (bind _sw (`self.SW`))
  (bind _se (`self.SE`))
  (bind _n (`self.N`))
  ;[1 1 1] Prend la position des points cardinaux et les multiplie par la distance souhaitée
  (`SceneComponent.K2_SetWorldLocation` _n (* (`SceneComponent.K2_GetComponentLocation` _n) (`self.Distance`)) false false)
  (`SceneComponent.K2_SetWorldLocation` _s (* (`SceneComponent.K2_GetComponentLocation` _s) (`self.Distance`)) false false)
  (`SceneComponent.K2_SetWorldLocation` _e (* (`SceneComponent.K2_GetComponentLocation` _e) (`self.Distance`)) false false)
  (`SceneComponent.K2_SetWorldLocation` _w (* (`SceneComponent.K2_GetComponentLocation` _w) (`self.Distance`)) false false)
  (`SceneComponent.K2_SetWorldLocation` _ne (* (`SceneComponent.K2_GetComponentLocation` _ne) (`self.Distance`)) false false)
  (`SceneComponent.K2_SetWorldLocation` _nw (* (`SceneComponent.K2_GetComponentLocation` _nw) (`self.Distance`)) false false)
  (`SceneComponent.K2_SetWorldLocation` _sw (* (`SceneComponent.K2_GetComponentLocation` _sw) (`self.Distance`)) false false)
  (`SceneComponent.K2_SetWorldLocation` _se (* (`SceneComponent.K2_GetComponentLocation` _se) (`self.Distance`)) false false)
  (return))

(fn `UserConstructionScript`
  (`self.SetDirectionDistance`))