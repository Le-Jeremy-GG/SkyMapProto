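; Star manager that builds the constellations and keeps star and constellation positions in step with the observer's date and location.
; On BeginPlay it spawns one BP_Constellation per DT_Constellations row, doubles the scale of its member stars and passes it the row data and star list.
; Date and time zone refresh events update UTC time or observer latitude/longitude, then recompute star positions and signal every constellation to refresh.
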(event `self.ReceiveBeginPlay`
  ;[1 1 1] Initialise les constellations
  (`self.SetConstellationStars`))

(event `/Game/Main/Constellations/Interfaces/BPI_Astro.Astro_RefreshDate`
  (params (CurrentDate :type "DateTime Structure"))
  ;[1 1 1] Actualise la date
  (set `self.UTCTime` CurrentDate)
  ;[1 1 1] Met a jour la position des etoiles et des constellations
  (`self.UpdateAllStarPositions` (`self.StarCalculationMethod`) :!label _label)
  (`self.UpdateConstellations`))

(event `/Game/Main/Constellations/Interfaces/BPI_Astro.Astro_RefreshTimeZone`
  (params (NewTimeZone :type "/Game/Main/Constellations/Datas/Struct_TimeZones Structure"))
  ;[1 1 1] Actualise les coordonnées Geographiques
  (setmembers `Observer` :`StructRef` (`self.Observer`) :`SurfaceLocation` (make `EarthSurfaceLocation` NewTimeZone_Latitude_8_B5DD237E43CC47BB168226BB118EA962 NewTimeZone_Longitude_9_BA465D284D1D0B7FCFC864A3CEA31C97))
  (goto _label))

(fn `SetConstellationStars`
  (locals (StarListPerConstellation :type "Array of Actor Object Reference") (ConstellationsDatas :type "Array of /Game/Main/Constellations/Datas/Struct_Constellation Structure"))
  (bind _constellationsdatas (`local.ConstellationsDatas`))
  ;[1 1 1] Cree les constellations
  (bind _outrownames (`DataTableFunctionLibrary.GetDataTableRowNames` "/Game/Main/Constellations/Datas/DT_Constellations.DT_Constellations"))
  (for _array_element _outrownames
    (bind _returnvalue (`|GetDataTableRow` "/Game/Main/Constellations/Datas/DT_Constellations.DT_Constellations" _array_element)
      (:`then`
        (bind _returnvalue_2 (`KismetArrayLibrary.Array_Add` (`local.ConstellationsDatas`) _returnvalue))
        (bind _returnvalue_3 (`|SpawnActorFromClass` "/Game/Main/Constellations/Blueprints/BP_Constellation.BP_Constellation_C" (`KismetMathLibrary.MakeTransform` (0.0 0.0 0.0)) "Undefined" "OverrideRootScale" null null))
        (bind _returnvalue_4 (`KismetArrayLibrary.Array_Add` (`self.ConstellationManagers`) _returnvalue_3))
        (bind (_output_constellationname _output_description _output_degrees _output_starnamehr) (break `/Game/Main/Constellations/Datas/Struct_Constellation` (`|GetArrayItem` _constellationsdatas _returnvalue_2)))
        ;[1 1 1] Liste les etoiles des constellations et les aggrandit pour les demarquer des autres
        (for _array_element_2 _output_starnamehr
          (bind _staractor (`self.FindStarByRowNameKey` _array_element_2))
          (`self.SetActorScale3D` _staractor (* (`self.GetActorScale3D` _staractor) 2.0))
          (`KismetArrayLibrary.Array_Add` (`local.StarListPerConstellation`) _staractor))
        (message `/Game/Main/Constellations/Interfaces/BPI_Stars.Constell_SetConstellation` (`|GetArrayItem` (`self.ConstellationManagers`) _returnvalue_4) (`|GetArrayItem` _constellationsdatas _returnvalue_2) (`local.StarListPerConstellation`))
        (`KismetArrayLibrary.Array_Clear` (`local.StarListPerConstellation`)))))
  (return))

(fn `UpdateConstellations`
  ;[1 1 1] Envoie le signal aux Constellation Managers de mettre a jour leurs positions.
  (for _array_element (`self.ConstellationManagers`)
    (message `/Game/Main/Constellations/Interfaces/BPI_Stars.RefreshConstellations` _array_element))
  (return))

(fn `UserConstructionScript`)