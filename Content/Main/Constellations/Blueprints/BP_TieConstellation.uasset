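; Constellation link actor that draws a tie from its assigned star to a target star and labels that star with its international name.
; RefreshConstellations stretches and aims the tie between both stars, or collapses it without a target, and turns the label toward the player.
; Hover and visibility toggles go through ConstellationManager.
; ConstellSetOpacity picks a target opacity, which a looping timer eases toward on a dynamic material.
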(event `/Game/Main/Constellations/Interfaces/BPI_Stars.Constell_SetOpacity`
  (params (Visible :type Boolean) (Hovered :type Boolean))
  (`KismetSystemLibrary.K2_ClearTimer` null "OpacityTimer")
  ;[1 1 1] Regle opacite si survole
  (if Hovered
    (if Visible
      (set `self.AlphaOpacity` 0.02)
      (else
        (set `self.AlphaOpacity` 0.002)))
    (else
      ;[1 1 1] Regle l'Opacité du lien
      (if Visible
        (set `self.AlphaOpacity` 0.2)
        (else
          (set `self.AlphaOpacity` 0.002)))))
  (`KismetSystemLibrary.K2_SetTimer` null "OpacityTimer" 0.05 true))

(event `self.ReceiveBeginPlay`
  ;[1 1 1] Begin Play
  ;[1 1 1] Cree un materiau dynamique pr controler l'opacité du lien
  (bind _returnvalue (`KismetMaterialLibrary.CreateDynamicMaterialInstance` "/Game/Main/Constellations/Materials/M_StarTie.M_StarTie"))
  (bind _output_get (set `self.StarMat` _returnvalue))
  (`PrimitiveComponent.SetMaterial` (`self.Cube`) 0 _output_get)
  (`MaterialInstanceDynamic.SetScalarParameterValue` (`self.StarMat`) "Opacity" 0.002))

(event `/Game/Main/Constellations/Interfaces/BPI_Stars.TieConstell_SetAssignedStar`
  (params (AssignedStar :type "Actor Object Reference") (StarToAim :type "Actor Object Reference") (ConstellationManager :type "Actor Object Reference") (StarName :type "/Game/Main/Constellations/Datas/Struct_StarName Structure") (Index :type Integer))
  ;[1 1 1] Recupere l'etoile qui est assignée au lien et son nom
  (set `self.AssignedStar` AssignedStar)
  (set `self.StarToAim` (select `bool` (`KismetSystemLibrary.IsValid` StarToAim) :`true` StarToAim))
  (set `self.ConstellationManager` ConstellationManager)
  (set `self.StarName` StarName)
  (set `self.StarIndex` Index)
  (`self.SetStarName`))

(event `/Game/Main/Constellations/Interfaces/BPI_Stars.Constell_SetHovered`
  (params (Visible :type Boolean))
  (message `/Game/Main/Constellations/Interfaces/BPI_Stars.Constell_SetOpacity` (`self.ConstellationManager`) Visible true))

(event `/Game/Main/Constellations/Interfaces/BPI_Stars.RefreshConstellations`
  (bind _textrender (`self.TextRender`))
  ;[1 1 1] Qd appelée, replace le lien entre les etoiles a lier
  (`self.RefreshTransforms`)
  ;[1 1 1] Puis replace le nom de l'etoile assignée
  (`SceneComponent.K2_SetWorldLocation` _textrender (`SceneComponent.K2_GetComponentLocation` (`self.Scene`)) false false)
  (`SceneComponent.K2_SetWorldRotation` _textrender (`KismetMathLibrary.FindLookAtRotation` (`SceneComponent.K2_GetComponentLocation` _textrender) (`self.K2_GetActorLocation` (`GameplayStatics.GetPlayerPawn` 0))) false false))

(event `/Game/Main/Constellations/Interfaces/BPI_Stars.TieConstell_DisplayConstell`
  ;[1 1 1] TieConstell
  (if (`self.Visibility`)
    (set `self.Visibility` false)
    (else
      (set `self.Visibility` true)))
  (message `/Game/Main/Constellations/Interfaces/BPI_Stars.Constell_SetOpacity` (`self.ConstellationManager`) (`self.Visibility`) false))

(fn `OpacityTimer`
  ;[1 1 1] Lerp jusqu'à l'opacity voulue
  (bind _returnvalue (`MaterialInstanceDynamic.K2_GetScalarParameterValue` (`self.StarMat`) "Opacity"))
  (if (not (`KismetMathLibrary.NearlyEqual_FloatFloat` _returnvalue (`self.AlphaOpacity`) 0.05))
    (`MaterialInstanceDynamic.SetScalarParameterValue` (`self.StarMat`) "Opacity" (`KismetMathLibrary.Lerp` _returnvalue (`self.AlphaOpacity`) (select `bool` (> (`self.AlphaOpacity`) _returnvalue) :`false` (+ _returnvalue -0.025) :`true` (+ _returnvalue 0.025))))
    (else
      (`MaterialInstanceDynamic.SetScalarParameterValue` (`self.StarMat`) "Opacity" (`self.AlphaOpacity`))
      (`KismetSystemLibrary.K2_ClearTimer` null "OpacityTimer")))
  (return))

(fn `RefreshTransforms`
  (bind _tiebasedimension (`self.TieBaseDimension`))
  (bind _tiebasedimension_2 (`self.TieBaseDimension`))
  (bind _returnvalue (`self.K2_GetActorLocation` (`self.StarToAim`)))
  (bind _returnvalue_2 (`self.K2_GetActorLocation` (`self.AssignedStar`)))
  (`/Engine/EditorBlueprintResources/StandardMacros.IsValid` (`self.StarToAim`)
    (:`Is Valid`
      (`SceneComponent.K2_SetWorldTransform` (`self.Scene`) (`KismetMathLibrary.MakeTransform` _returnvalue_2 (`KismetMathLibrary.FindLookAtRotation` _returnvalue_2 _returnvalue) (`KismetMathLibrary.MakeVector` (/ (`KismetMathLibrary.VSize` (- _returnvalue _returnvalue_2)) 100.0) _tiebasedimension _tiebasedimension)) false false))
    (:`Is Not Valid`
      (`SceneComponent.K2_SetWorldTransform` (`self.Scene`) (`KismetMathLibrary.MakeTransform` _returnvalue_2 (struct) (`KismetMathLibrary.MakeVector` _tiebasedimension_2 _tiebasedimension_2 _tiebasedimension_2)) false false)))
  (`SceneComponent.K2_SetWorldLocation` (`self.Sphere`) _returnvalue_2 false false)
  (return))

(fn `SetStarName`
  ;[1 1 1] Affiche le nom tahitien ainsi que le nom international entre parenthese
  (`TextRenderComponent.K2_SetText` (`self.TextRender`) (`KismetTextLibrary.Conv_StringToText` (`.StarNameInternational_27_038E1AF7493A653A1FB3F1BBEA86698F` (break `/Game/Main/Constellations/Datas/Struct_StarName` (`self.StarName`)))))
  (return))

(fn `UserConstructionScript`)