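; Time manager for the constellations scene: advances a UTC date by timer, pushes it to all BPI_Astro actors and shows local time on clock and calendar widgets (screen or VR).
; Calendar jumps fast-forward with distance-scaled GameMode speed, locking the Sun at night and stepping by days on long forward spans.
; Vertical controller movement scrubs time within the current day.
; Time zone presets from DT_TimeZones set the astros' observation point.
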(event `self.ReceiveBeginPlay`
  (bind _vr (`self.VR`))
  ;[1 1 1] BeginPlay
  ;[1 1 1] Recupere le Temps universel actuel et demarre le cycle du temps
  (set `self.CurrentDate` (`KismetMathLibrary.UtcNow`))
  (`self.InitializeCycle` 1.0)
  ;[1 1 1] Set le Calendrier et l'horloge
  (bind _returnvalue (`|CreateWidget` "/Game/Main/Constellations/UserInterfaces/WBP_TimeOfDay.WBP_TimeOfDay_C"))
  (bind _output_get (set `self.TimeOfDay` _returnvalue))
  (`self.SetWidgetForScreenOrVR` _output_get (`self.wTimeOfDay`) _vr)
  (bind _returnvalue_2 (`|CreateWidget` "/Game/Main/Constellations/UserInterfaces/WBP_Calendar.WBP_Calendar_C" null (`self.CurrentDate`) self))
  (bind _output_get_2 (set `self.Calendar` _returnvalue_2))
  (`self.SetWidgetForScreenOrVR` _output_get_2 (`self.wCalendar`) _vr)
  ;[1 1 1] Récupère les astres qui s'aligneront sur le temps. Ils ont tous l'interface "Astro"
  (bind _outactors (`GameplayStatics.GetAllActorsWithInterface` "/Game/Main/Constellations/Interfaces/BPI_Astro.BPI_Astro_C"))
  (for _array_element _outactors
    (`KismetArrayLibrary.Array_Add` (`self.AstroObjects`) _array_element))
  ;[1 1 1] Set la timezone des astres
  (`self.SetNewTimeZone` (`self.TimeZone`)))

(event `/Game/Main/Constellations/Interfaces/BPI_Time.TimeManagerReverseHandling`
  (params (Reverse :type Boolean))
  ;[1 1 1] ReverseTheHandling
  (set `self.Reverse` Reverse))

(event `/Game/Main/Constellations/Interfaces/BPI_Time.SetTimeSpeed`
  (params (Speed :type "Float (single-precision)"))
  ;[1 1 1] Recuperer la vitesse de jeu qd elle est mise a jour dans le GM
  (set `self.Speed` Speed))

(event `/Game/Main/Constellations/Interfaces/BPI_Time.TimeManager_HandleTime`
  (params (Handle :type Boolean) (Controller :type "SceneComponent Object Reference"))
  ;[1 1 1] Qd les gachettes sont préssées ou relachées depuis le controleur, synchronise le temps sur le Handling
  (if (`self.bIsFastForwarding`)
    _
    (elif Handle
      (`self.StartTimeHandle` Controller)
      (else
        (`self.StopTimeHandle`)))))

(fn `AddDay`
  (returns (NewDate :type "DateTime Structure"))
  ;[1 1 1] Appelée dans le Timer, recupere la variable Speed representant alors un nombre de secondes,
  ; et l'additionne a la date actuelle
  (return (+ (`self.CurrentDate`) (`KismetMathLibrary.MakeTimespan` 1))))

(fn `AddSecond`
  (returns (NewDate :type "DateTime Structure"))
  ;[1 1 1] Appelée dans le Timer, recupere la variable Speed representant alors un nombre de secondes,
  ; et l'additionne a la date actuelle
  (return (+ (`self.CurrentDate`) (`KismetMathLibrary.MakeTimespan` 0 0 0 (`KismetMathLibrary.FTrunc` (`self.Speed`))))))

(fn `CheckFastForward`
  (bind _returnvalue (- (`self.DateToGo`) (`self.CurrentDate`)))
  (bind _isnight (`self.CheckIfNight` (`/Game/Main/BFL_UTC.UTCToLocal` (`self.CurrentDate`) (`self.TimeZone`))))
  (bind _returnvalue_2 (`KismetMathLibrary.GetTotalDays` _returnvalue))
  (bind _returnvalue_3 (* (`KismetMathLibrary.Abs` _returnvalue_2) 2000.0))
  ;[1 1 1] Si la date actuelle est assez proche de celle visée, stoppe le fast forward et va direct à la date souhaitée
  (if (< (`KismetMathLibrary.Abs` (`KismetMathLibrary.GetTotalMinutes` _returnvalue)) 5.0)
    (`self.Stop Fast Forward` (`self.DateToGo`))
    (return)
    (else
      ;[1 1 1] Multiplie vitesse du fast forward par la durée restante à parcourir afin que le temps de Fast Forward reste le meme peu importe qu'on remonte de 3 jours ou 3 ans
      (message `/Game/Main/Constellations/Interfaces/BPI_GMConstell.GM_SetWorldSpeed` (`GameplayStatics.GetGameMode`) (* (`KismetMathLibrary.SelectFloat` 1.0 -1.0 (>= _returnvalue_2 0.0)) (`KismetMathLibrary.SelectFloat` (`KismetMathLibrary.SelectFloat` 2000.0 _returnvalue_3 (and (not (`self.bIsSunLocked`)) (> (`KismetMathLibrary.Abs` (`KismetMathLibrary.GetTotalHours` (- (`self.DateToGo`) (`self.CurrentDate`)))) 24.0))) 250.0 (> _returnvalue_3 500.0))))
      ;[1 1 1] Si la duree restante est trop grande et que donc le temps passe trop vite, verouille le soleil a minuit afin de ne pas avoir le cycle jour nuit qui s'emballe
      (if (> (`KismetMathLibrary.Abs` (`KismetMathLibrary.GetTotalHours` (- (`self.DateToGo`) (`self.CurrentDate`)))) 24.0)
        (if (and (not (`self.bIsSunLocked`)) _isnight)
          (set `self.bIsSunLocked` true)
          (message `/Game/Main/Constellations/Interfaces/BPI_Astro.Astro_Lock` (`self.Sun`) true (`KismetMathLibrary.GetHour` (`self.CurrentDate`))))
        (elif (and _isnight (`self.bIsSunLocked`))
          (set `self.bIsSunLocked` false)
          (message `/Game/Main/Constellations/Interfaces/BPI_Astro.Astro_Lock` (`self.Sun`) false -1)))
      ;[1 1 1] Set le fast forward par jour
      (if (and (not (`self.bIsFastFowardingDay`)) (> (`KismetMathLibrary.GetTotalDays` (- (`self.DateToGo`) (`self.CurrentDate`))) 3.0) (`self.bIsSunLocked`))
        (set `self.bIsFastFowardingDay` true)
        (elif (and (`self.bIsFastFowardingDay`) (<= (`KismetMathLibrary.GetTotalDays` (- (`self.DateToGo`) (`self.CurrentDate`))) 2.0))
          (set `self.bIsFastFowardingDay` false)))
      (return))))

(fn `CheckIfNight`
  (params (Date :type "DateTime Structure"))
  (returns (IsNight :type Boolean))
  (bind (_year _month _day _hour) (`KismetMathLibrary.BreakDateTime` Date))
  (return (or (and (>= _hour 20) (`KismetMathLibrary.IsAfternoon` Date)) (and (`KismetMathLibrary.IsMorning` Date) (<= _hour 5)))))

(fn `DayCycle_Timer`
  (if (`self.bIsFastForwarding`)
    ;[1 1 1] Si en fast forward, controle celui-ci.
    (`self.CheckFastForward`)
    (if (`self.bIsFastFowardingDay`)
      (bind _newdate (`self.AddDay`))
      (`self.RefreshTimeofDay` _newdate)
      (else
        ;[1 1 1] Met a jour la date en lui ajoutant le temps qui s'est écoulé depuis le dernier interval (celui de la variable Speed)
        (bind _newdate_2 (`self.AddSecond` :!label _label))
        (`self.RefreshTimeofDay` _newdate_2)))
    (else
      (goto _label)))
  (return))

(fn `GetPredefinedTimeZone`
  (params (TimeZone :type "/Game/Main/Constellations/Datas/Enum_TimeZones Enum" :default "NewEnumerator0"))
  (returns (UTC :type "Float (double-precision)"))
  ;[1 1 1] Recupere le decalage horaire par rapport au temps international coordonnée.
  (bind _returnvalue (`|GetDataTableRow` "/Game/Main/Constellations/Datas/DT_TimeZones.DT_TimeZones" (select `/Game/Main/Constellations/Datas/Enum_TimeZones` TimeZone :`NewEnumerator0` "Tahiti" :`NewEnumerator1` "HivaOa" :`NewEnumerator2` "Hawai" :`NewEnumerator3` "NewZealand" :`NewEnumerator4` "RapaNui" :`NewEnumerator5` "NewCaledonia" :!type "Name"))
    (:`then`
      (return (`.TimeZone_11_9A354EC140D07EC0EE8FF9A3559B54BD` (break `/Game/Main/Constellations/Datas/Struct_TimeZones` _returnvalue))))))

(fn `HandleTime_Timer`
  (bind (_currentdate_year _currentdate_month _currentdate_day) (`KismetMathLibrary.BreakDateTime` (`self.CurrentDate`)))
  (bind (_controllerpreviouslocation_x _controllerpreviouslocation_y _controllerpreviouslocation_z) (`KismetMathLibrary.BreakVector` (`self.ControllerPreviousLocation`)))
  (bind _returnvalue (* (- (.z (`SceneComponent.RelativeLocation` (`self.ControllerHandling`))) _controllerpreviouslocation_z) 10.0))
  (bind (_year _month _day _hour _minute _second _millisecond) (`KismetMathLibrary.BreakDateTime` (+ (`self.CurrentDate`) (`KismetMathLibrary.MakeTimespan` 0 0 (`KismetMathLibrary.FTrunc` (`KismetMathLibrary.SelectFloat` (* _returnvalue -1.0) _returnvalue (`self.Reverse`)))))))
  ;[1 1 1] Convertit la direction en minutes à ajouter ou soustraire à la journée actuelle
  (`self.RefreshTimeofDay` (`KismetMathLibrary.MakeDateTime` _currentdate_year _currentdate_month _currentdate_day _hour _minute _second _millisecond))
  ;[1 1 1] Retient la position actuelle du controlleur afin de la comparer à la prochaine et pouvoir recalculer la direction
  (set `self.ControllerPreviousLocation` (`SceneComponent.RelativeLocation` (`self.ControllerHandling`)))
  (return))

(fn `InitializeCycle`
  (params (LoopDuration :type "Float (double-precision)"))
  ;[1 1 1] Initialise le Timer qui se declenche selon l'interval prédéfinie
  (`KismetSystemLibrary.K2_ClearTimer` null "DayCycle_Timer")
  (`KismetSystemLibrary.K2_SetTimer` null "DayCycle_Timer" LoopDuration true)
  (return))

(fn `InitializeFastForward`
  (params (DateToGo :type "DateTime Structure"))
  ;[1 1 1] Passe en mode Fast Forward
  (set `self.bIsFastForwarding` true)
  ;[1 1 1] La date choisie dans le calendrier est en temps local, donc je m'assure de la convertir en temps international
  (set `self.DateToGo` (`/Game/Main/BFL_UTC.LocalToUTC` DateToGo (`self.TimeZone`)))
  ;[1 1 1] Reset le Timer avec un interval plus court, au lieu d'une seconde
  (`self.InitializeCycle` 0.05)
  ;[1 1 1] Une fois le fast forward lancé, verouille les commandes que l'utilisateur n'est plus censé devoir utiliser
  (`/Game/Main/Constellations/UserInterfaces/WBP_Calendar.FastForwardMode` (`self.Calendar`) true)
  (set `self.bIsSunLocked` false)
  (return))

(fn `RefreshAstroDate`
  (params (CurrentDate :type "DateTime Structure"))
  ;[1 1 1] Actualise la date de tous les astres listés
  (for _array_element (`self.AstroObjects`)
    (message `/Game/Main/Constellations/Interfaces/BPI_Astro.Astro_RefreshDate` _array_element CurrentDate))
  (return))

(fn `RefreshAstroTimeZone`
  (params (NewTimeZone :type "/Game/Main/Constellations/Datas/Struct_TimeZones Structure"))
  ;[1 1 1] Envoie les nouvelles coordonnées geographiques aux astres afin de modifier leur point d'observation.
  (for _array_element (`self.AstroObjects`)
    (message `/Game/Main/Constellations/Interfaces/BPI_Astro.Astro_RefreshTimeZone` _array_element NewTimeZone))
  (return))

(fn `RefreshTimeofDay`
  (params (NewDate :type "DateTime Structure"))
  ;[1 1 1] Set la date et l'envoie aux astres pour actualiser leurs positions
  (bind _output_get (set `self.CurrentDate` NewDate))
  (`self.RefreshAstroDate` _output_get)
  ;[1 1 1] Converti le temps international en tmps local pr l'afficher à l'horloge
  (`/Game/Main/Constellations/UserInterfaces/WBP_TimeOfDay.SetClock` (`self.TimeOfDay`) (`/Game/Main/BFL_UTC.UTCToLocal` (`self.CurrentDate`) (`self.TimeZone`)))
  (return))

(fn `SetNewTimeZone`
  (params (Location :type "/Game/Main/Constellations/Datas/Enum_TimeZones Enum" :default "NewEnumerator0"))
  ;[1 1 1] Recupere les données de l'endroit choisi (latitude, longitude, fuseau horaire) et les envoie aux astres pour qu'ils se mettent à jour
  (bind _output_get (set `self.TimeZone` Location))
  (bind _returnvalue (`|GetDataTableRow` "/Game/Main/Constellations/Datas/DT_TimeZones.DT_TimeZones" (select `/Game/Main/Constellations/Datas/Enum_TimeZones` _output_get :`NewEnumerator0` "Tahiti" :`NewEnumerator1` "HivaOa" :`NewEnumerator2` "Hawai" :`NewEnumerator3` "NewZealand" :`NewEnumerator4` "RapaNui" :`NewEnumerator5` "NewCaledonia" :!type "Name"))
    (:`then`
      (`self.RefreshAstroTimeZone` _returnvalue))
    (:`RowNotFound`
      (`KismetSystemLibrary.PrintString` "TIMEZONE NOT FOUND" true true (struct :`R` 1.0 :`B` 0.036017 :`A` 1.0))))
  (return))

(fn `SetWidgetForScreenOrVR`
  (params (WidgetToSet :type "UserWidget Object Reference") (`3DWidgetForVR` :type "WidgetComponent Object Reference") (VR :type Boolean))
  (bind _returnvalue (`GameplayStatics.GetPlayerController` 0))
  (if VR
    ;[1 1 1] Si en VR, se synchronise sur les Widget Components
    (`WidgetComponent.SetWidget` `3DWidgetForVR` WidgetToSet)
    (return)
    (else
      ;[1 1 1] Sinon, cache les Widget Components et affiche directement les widgets a l'ecran (et active le curseur)
      (`UserWidget.AddToViewport` WidgetToSet 0)
      (`SceneComponent.SetVisibility` `3DWidgetForVR` false false)
      (set `PlayerController.bEnableClickEvents` true _returnvalue)
      (set `PlayerController.bShowMouseCursor` true _returnvalue)
      (return))))

(fn `StartTimeHandle`
  (params (Controller :type "SceneComponent Object Reference"))
  ;[1 1 1] Recupere le controlleur pr retenir sa position
  (set `self.ControllerHandling` Controller)
  ;[1 1 1] Stoppe l'ecoulement du temps, celui-ci etant maintenant controlé par le Handling
  (message `/Game/Main/Constellations/Interfaces/BPI_GMConstell.GM_SetWorldSpeed` (`GameplayStatics.GetGameMode`) 0.0)
  ;[1 1 1] Recupere une premiere fois la position du controlleur
  (set `self.ControllerPreviousLocation` (`SceneComponent.RelativeLocation` (`self.ControllerHandling`)))
  ;[1 1 1] Lance le timer qui va verifier dans quelle direction on bouge le controlleur
  (`KismetSystemLibrary.K2_SetTimer` null "HandleTime_Timer" 0.025 true)
  (return))

(fn `Stop Fast Forward`
  (params (NewDate :type "DateTime Structure"))
  (set `self.bIsFastForwarding` false)
  (set `self.bIsSunLocked` false)
  (set `self.bIsFastFowardingDay` false)
  ;[1 1 1] Sort du mode FF et réinitialise le Timer pour qu'il se declenche  à nouveau qu'une fois par seconde
  (`self.InitializeCycle` 1.0)
  ;[1 1 1] Permet au joueur d'acceder a nouveau au calendrier
  (`/Game/Main/Constellations/UserInterfaces/WBP_Calendar.FastForwardMode` (`self.Calendar`) false)
  ;[1 1 1] Reset la vitesse par defaut dans le GM
  (message `/Game/Main/Constellations/Interfaces/BPI_GMConstell.GM_SetWorldSpeed` (`GameplayStatics.GetGameMode`) 1.0)
  ;[1 1 1] Deverrouille le soleil au cas ou
  (message `/Game/Main/Constellations/Interfaces/BPI_Astro.Astro_Lock` (`self.Sun`) false -1)
  ;[1 1 1] Set la date actuelle à celle souhaitée afin d'etre précis
  (`self.RefreshTimeofDay` NewDate)
  (return))

(fn `StopTimeHandle`
  ;[1 1 1] Arrete le Handling et retabli l'ecoulement du temps
  (`KismetSystemLibrary.K2_ClearTimer` null "HandleTime_Timer")
  (set `self.ControllerHandling` null)
  (message `/Game/Main/Constellations/Interfaces/BPI_GMConstell.GM_SetWorldSpeed` (`GameplayStatics.GetGameMode`) 1.0)
  (return))

(fn `UserConstructionScript`)