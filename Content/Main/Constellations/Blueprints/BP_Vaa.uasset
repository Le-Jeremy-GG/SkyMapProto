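; BP_Vaa is a pirogue (va'a) actor meant to sail between Departure and Destination points according to the time of day.
; BeginPlay measures the travel distance and starts a looping timer.
; CheckPositionFromHour converts the TimeManager's UTC date to local time and tests whether it falls between departure and destination hours.
; It is unfinished: the check drives nothing, and return-trip and interpolation nodes are unconnected.
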(event `self.ReceiveBeginPlay`
  (set `self.TravelDistance` (`KismetMathLibrary.VSize` (- (`SceneComponent.K2_GetComponentLocation` (`self.Departure`)) (`SceneComponent.K2_GetComponentLocation` (`self.Destination`)))))
  (`KismetSystemLibrary.K2_SetTimerDelegate` (`|CreateDelegate` :!event `CheckPositionFromHour`) 0.1 true))

(fn `CheckPositionFromHour`
  (locals (Date :type "Timespan Structure") (LocalDeparture :type "Timespan Structure") (LocalDestination :type "Timespan Structure"))
  (bind _timemanager (`self.TimeManager`))
  (bind (_local_year _local_month _local_day _local_hour _local_minute _local_second _local_millisecond) (`KismetMathLibrary.BreakDateTime` (`/Game/Main/BFL_UTC.UTCToLocal` (`/Game/Main/Constellations/Blueprints/BP_TimeManager.CurrentDate` _timemanager) (`/Game/Main/Constellations/Blueprints/BP_TimeManager.TimeZone` _timemanager))))
  (set `local.Date` (`KismetMathLibrary.MakeTimespan` _local_day _local_hour _local_minute _local_second _local_millisecond))
  (set `local.LocalDeparture` (`KismetMathLibrary.MakeTimespan` (`KismetMathLibrary.BreakTimespan` (`local.Date`)) (`self.DepartureHour`)))
  ;[1 1 1] Verifie si pirogue navigue
  (set `local.LocalDestination` (`KismetMathLibrary.MakeTimespan` (`KismetMathLibrary.BreakTimespan` (`local.Date`)) (`self.DestinationHour`)))
  (if (and (> (`local.Date`) (`local.LocalDeparture`)) (< (`local.Date`) (`local.LocalDestination`)))
    _))

(fn `UserConstructionScript`)