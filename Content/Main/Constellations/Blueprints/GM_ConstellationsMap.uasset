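; Game mode for the Constellations map that owns the world time speed and fades the view in from black at start.
; On BeginPlay it caches every actor implementing BPI_Time and pushes the default speed to them.
; SetSpeed writes the speed to the MPC_Speed parameter collection for animated materials like clouds and sea, then messages the cached actors.
; GMSetWorldSpeed lets callers change it, typically the calendar for fast forward.
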(event `self.ReceiveBeginPlay`
  ;[1 1 1] BeginPlay
  (`PlayerCameraManager.SetManualCameraFade` :`self` (`GameplayStatics.GetPlayerCameraManager` 0) :`InFadeAmount` 1.0 :`bInFadeAudio` true)
  ;[1 1 1] Liste tous les acteurs qui gerent le temps et qui ont besoin de recuperer la variable Speed (n'implique que le Time Manager pr le moment mais on sait jamais)
  (bind _outactors (`GameplayStatics.GetAllActorsWithInterface` "/Game/Main/Constellations/Interfaces/BPI_Time.BPI_Time_C"))
  (for _array_element _outactors
    (`KismetArrayLibrary.Array_Add` (`self.TimeActors`) _array_element))
  ;[1 1 1] ...Puis leur envoie la speed par defaut une premiere fois (on sait jamais)
  (`self.SetSpeed` (`self.Speed`))
  (`KismetSystemLibrary.Delay` 1.0)
  (`PlayerCameraManager.StartCameraFade` :`self` (`GameplayStatics.GetPlayerCameraManager` 0) :`FromAlpha` 1.0 :`Duration` 1.0 :`bShouldFadeAudio` true :`bHoldWhenFinished` true))

(event `/Game/Main/Constellations/Interfaces/BPI_GMConstell.GM_SetWorldSpeed`
  (params (NewSpeed :type "Float (single-precision)"))
  ;[1 1 1] Appelé lorsque la vitesse doit etre mise a jour.
  ; Generalement depuis le calendrier pour le Fast Forward
  (`self.SetSpeed` NewSpeed))

(fn `SetSpeed`
  (params (Speed :type "Float (double-precision)"))
  (bind _output_get (set `self.Speed` Speed))
  ;[1 1 1] Accorde la vitesse de base des materials qui bougent (nuages, mer) sur la vitesse set ici
  (`KismetMaterialLibrary.SetScalarParameterValue` "/Game/Main/Materials/MPC_Speed.MPC_Speed" "TimeSpeed" _output_get)
  ;[1 1 1] Envoie la valeur de Speed aux acteurs listés
  (for _array_element (`self.TimeActors`)
    (message `/Game/Main/Constellations/Interfaces/BPI_Time.SetTimeSpeed` _array_element (`self.Speed`)))
  (return))

(fn `UserConstructionScript`)