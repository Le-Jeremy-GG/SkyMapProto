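; Celestial body actor that places a planet or other body in the sky as seen from an Earth observer.
; Astro events update the observer's latitude/longitude or UTC time, then SetLocation recomputes the body's direction via PlanetDirectionFromEarth.
; The direction is normalized and scaled to a fixed distance from the world origin.
; AstroLock stores lock state, which date refresh ignores; LockToGivenHour separately overrides the hour and repositions.
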(event `/Game/Main/Constellations/Interfaces/BPI_Astro.Astro_Lock`
  (params (Lock :type Boolean) (HourToLock :type Integer))
  ;[1 1 1] Verouille l'astre
  (set `self.bIsLocked` Lock)
  (if (!= HourToLock -1)
    (set `self.HourToLock` HourToLock)))

(event `/Game/Main/Constellations/Interfaces/BPI_Astro.Astro_RefreshTimeZone`
  (params (NewTimeZone :type "/Game/Main/Constellations/Datas/Struct_TimeZones Structure"))
  ;[1 1 1] Mettre a jour coordonnées geographiques  et positionner l'astre en consequence
  (setmembers `Observer` :`StructRef` (`self.Observer`) :`SurfaceLocation` (make `EarthSurfaceLocation` NewTimeZone_Latitude_8_B5DD237E43CC47BB168226BB118EA962 NewTimeZone_Longitude_9_BA465D284D1D0B7FCFC864A3CEA31C97))
  (`self.SetLocation`))

(event `/Game/Main/Constellations/Interfaces/BPI_Astro.Astro_RefreshDate`
  (params (CurrentDate :type "DateTime Structure"))
  ;[1 1 1] Mettre a jour la date actuelle et positionner l'astre en consequence. Sauf si l'astre est verrouillé
  (set `self.UTCTime` CurrentDate)
  (`self.SetLocation`))

(fn `GetLocation`
  (returns (HorizonBodyLocation :type "AstroDoubleVector Structure"))
  (bind (_outdirection _outaz _outel _outdistance) (`AstroLibBPLibrary.PlanetDirectionFromEarth` (`self.Body`) (`self.Observer`) (`self.UTCTime`) "NoRefractionCorrection" (`self.NorthAdjustment`)))
  (return (* _outdirection _outdistance)))

(fn `LockToGivenHour`
  (params (HourToLock :type Integer))
  (bind (_utctime_year _utctime_month _utctime_day) (`KismetMathLibrary.BreakDateTime` (`self.UTCTime`)))
  ;[1 1 1] S'il n'est pas déjà bloqué à l'heure souhaitée, l'y amène
  (set `self.UTCTime` (`KismetMathLibrary.MakeDateTime` _utctime_year _utctime_month _utctime_day HourToLock 1))
  (`self.SetLocation`)
  (return))

(fn `SetLocation`
  (returns (HorizonLocationInAU :type "AstroDoubleVector Structure"))
  (bind _horizonbodylocation (`self.GetLocation`))
  (`self.K2_SetActorLocation` (* (`KismetMathLibrary.Vector_NormalUnsafe` (`DoubleFunction.Conv_FAstroDoubleVectorToFVector` _horizonbodylocation)) (`self.UUDistanceFromOrigin`)))
  (return _horizonbodylocation))

(fn `UserConstructionScript`)