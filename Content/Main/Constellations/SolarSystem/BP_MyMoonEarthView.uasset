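; Moon actor for the solar system's view from Earth, extending a parent that computes and sets its location.
; Each location update yaws the actor by the north adjustment and refreshes eclipse and illumination lighting.
; Ecliptic Moon-to-Earth and Moon-to-Sun vectors in kilometers, plus a north-adjusted observer-based Moon-to-Sun direction, feed a shared material parameter collection.
; Construction applies a dynamic instance of the ground Moon material to the mesh.
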(event `self.ReceiveBeginPlay`
  (`parent.ReceiveBeginPlay`))

(fn `MoonToEarthGeocenter`
  (returns (MoonToEarthGeocenterInKM :type "AstroDoubleVector Structure"))
  (bind _location (`EphemerisManager.GetState` "Earth" "Moon" (`AstroLibBPLibrary.GetJulianDate` (`self.UTCTime`)) (struct) "Ecliptical"))
  (return (`AstroLibBPLibrary.GetKMFromAU` _location)))

(fn `MoonToSunCenter`
  (returns (MoonToSunInKM :type "AstroDoubleVector Structure"))
  (bind _location (`EphemerisManager.GetState` "Sun" "Moon" (`AstroLibBPLibrary.GetJulianDate` (`self.UTCTime`)) (struct) "Ecliptical"))
  (return (`AstroLibBPLibrary.GetKMFromAU` _location)))

(fn `SetLocation`
  (returns (HorizonLocationInAU :type "AstroDoubleVector Structure"))
  (bind _horizonlocationinau (`parent.SetLocation`))
  (`self.UpdateMoonLighting` _horizonlocationinau)
  (`self.K2_SetActorRotation` (`KismetMathLibrary.MakeRotator` 0.0 0.0 (`self.NorthAdjustment`)))
  (return _horizonlocationinau))

(fn `UpdateMoonLighting`
  (params (HorizonLocationInAU :type "AstroDoubleVector Structure"))
  (bind (_outdirection _outaz _outel _outdistance) (`AstroLibBPLibrary.PlanetDirectionFromEarth` "Sun" (`self.Observer`) (`self.UTCTime`)))
  ;[1 1 1] Eclipse lighting
  (bind _moontoearthgeocenterinkm (`self.MoonToEarthGeocenter`))
  (`KismetMaterialLibrary.SetVectorParameterValue` "/AstroLib/AstroLib/Materials/AstroMaterialCollection.AstroMaterialCollection" "MoonToEarthGeocenterInKM" (`DoubleFunction.Conv_FAstroDoubleVectorToLinearColor` _moontoearthgeocenterinkm))
  (bind _moontosuninkm (`self.MoonToSunCenter`))
  (`KismetMaterialLibrary.SetVectorParameterValue` "/AstroLib/AstroLib/Materials/AstroMaterialCollection.AstroMaterialCollection" "MoonToSunInKM" (`DoubleFunction.Conv_FAstroDoubleVectorToLinearColor` _moontosuninkm))
  ;[1 1 1] Lunar illumination
  (`KismetMaterialLibrary.SetVectorParameterValue` "/AstroLib/AstroLib/Materials/AstroMaterialCollection.AstroMaterialCollection" "MoonToSunDirection" (`DoubleFunction.Conv_FAstroDoubleVectorToLinearColor` (- (`DoubleFunction.RotateAngleAxisDblVec` (* _outdirection _outdistance) (`self.NorthAdjustment`) (0.0 0.0 1.0)) HorizonLocationInAU))))

(fn `UserConstructionScript`
  (`parent.UserConstructionScript`)
  (`PrimitiveComponent.CreateDynamicMaterialInstance` (`self.StaticMesh`) 0 "/AstroLib/AstroLib/Materials/GroundMoonMaterial.GroundMoonMaterial" "None"))