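; Sun actor for the Earth-view sky in the solar system, extending a parent astro object.
; On date refresh it either locks to a given hour (noted as midnight) or follows the parent's update.
; SetLocation feeds the Sun position to a material parameter collection for star visibility, aims the directional light at the origin and refreshes the SkySphere.
; WasLocked is set on lock, but its daytime-hold logic is disconnected.
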(event `/Game/Main/Constellations/Interfaces/BPI_Astro.Astro_RefreshDate`
  (params (CurrentDate :type "DateTime Structure"))
  ;[1 1 1] Amène le Soleil a minuit si IsLocked est vrai
  (if (`self.bIsLocked`)
    (`self.LockToGivenHour` (`self.HourToLock`))
    (else
      (`parent.Astro_RefreshDate` CurrentDate))))

(event `/Game/Main/Constellations/Interfaces/BPI_Astro.Astro_Lock`
  (params (Lock :type Boolean) (HourToLock :type Integer))
  ;[1 1 1] AstroLock
  (`parent.Astro_Lock` Lock HourToLock)
  (if Lock
    (set `self.WasLocked` true)))

(fn `SetLocation`
  (returns (HorizonLocationInAU :type "AstroDoubleVector Structure"))
  (locals (SunLocationLoc :type "AstroDoubleVector Structure"))
  (bind _skysphere (`self.SkySphere`))
  (bind _horizonlocationinau (`parent.SetLocation`))
  (set `local.SunLocationLoc` _horizonlocationinau)
  (`KismetMaterialLibrary.SetVectorParameterValue` "/AstroLib/AstroLib/Materials/AstroMaterialCollection.AstroMaterialCollection" "SunDirection" (`KismetMathLibrary.Conv_VectorToLinearColor` (`self.K2_GetActorLocation`)) :!pinned true) ; Turn stars on when sun sets
  (if (!= (`self.DirectionalLightActor`) null)
    (`self.K2_SetActorLocationAndRotation` (`self.DirectionalLightActor`) (`self.K2_GetActorLocation`) (`KismetMathLibrary.FindLookAtRotation` (`DoubleFunction.Conv_FAstroDoubleVectorToFVector` (`local.SunLocationLoc`)) (`KismetMathLibrary.MakeVector` 0.0)) false false)
    (if (!= (`self.SkySphere`) null)
      ;[1 1 1] Refresh SkySphere material
      (`/Engine/EngineSky/BP_Sky_Sphere.UpdateSunDirection` _skysphere)
      (set `/Engine/EngineSky/BP_Sky_Sphere.Refresh material` true _skysphere)
      (return (`local.SunLocationLoc`)))))

(fn `UserConstructionScript`
  (`parent.UserConstructionScript`))