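; BP_VolumetricWater is an actor that builds layered water by stacking BP_WaterTile actors, presumably to fake volume.
; On BeginPlay it spawns NbOfLayers tiles at its own X and Y, starting at its Z and stepping down by DistanceBetweenLayers.
; The construction script is empty, so the stack is created only at runtime, and the spawned tiles are not stored or updated afterward.
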(event `self.ReceiveBeginPlay`
  (bind (_returnvalue_x _returnvalue_y _returnvalue_z) (`KismetMathLibrary.BreakVector` (`self.K2_GetActorLocation`)))
  (bind (_returnvalue_x_2 _returnvalue_y_2) (`KismetMathLibrary.BreakVector` (`self.K2_GetActorLocation`)))
  (set `self.NextLayerLocation` _returnvalue_z)
  (for _ (range (`self.NbOfLayers`))
    (`|SpawnActorFromClass` "/Game/Main/Environments/Water/BP_WaterTile.BP_WaterTile_C" (`KismetMathLibrary.MakeTransform` (`KismetMathLibrary.MakeVector` _returnvalue_x_2 _returnvalue_y_2 (`self.NextLayerLocation`))) "Undefined" "OverrideRootScale" null null)
    (set `self.NextLayerLocation` (- (`self.NextLayerLocation`) (`self.DistanceBetweenLayers`)))))

(fn `UserConstructionScript`)