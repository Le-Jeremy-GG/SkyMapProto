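; BPC_FrontRopes is a front ropes piece of the Tipairua that can switch between a hologram look and its standard look.
; Its PiecesSwitchMaterial event takes an IsHologram flag and sets material slot 0 of the static mesh to one of two rope material instances.
; It has no other active logic, as BeginPlay, overlap and Tick are disabled stubs and the construction script only calls its parent.
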(event `/Game/Main/Tipairua/Blueprints/BPI_Vaa.Pieces_SwitchMaterial`
  (params (IsHologram :type Boolean))
  (if IsHologram
    (`PrimitiveComponent.SetMaterial` (`self.StaticMesh`) 0 "/Game/Main/Tipairua/Textures/MI_Tipairua_Ropes_2.MI_Tipairua_Ropes_2")
    (else
      (`PrimitiveComponent.SetMaterial` (`self.StaticMesh`) 0 "/Game/Main/Tipairua/Textures/MI_Tipairua_Ropes.MI_Tipairua_Ropes"))))

(fn `UserConstructionScript`
  (`parent.UserConstructionScript`))