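; A single piece of the vaa (pirogue) model in VR, which can be manipulated on its own when in exploded view.
; A looping timer lerps it to a given transform when the exploded state is set.
; When exploded, it handles hand attachment, two-hand move/rotate/scale with thumbstick offset, and joystick distance control.
; Otherwise it forwards those interactions to its parent actor, so the vaa responds as a whole.
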(event `self.ReceiveBeginPlay`
  (`NiagaraFunctionLibrary.OverrideSystemUserVariableStaticMeshComponent` null "ModuleSource" (`self.StaticMesh`)))

(event `/Game/Main/Tipairua/Blueprints/BPI_Vaa.Pieces_SetExplodedView`
  (params (bIsExploded :type Boolean) (GoTo :type "Transform Structure"))
  ;[1 1 1] Prepare le passage en vue eclatée ou ramene les pieces
  (set `self.bIsExploded` bIsExploded)
  (set `self.Destination` GoTo)
  (set `self.OriginalLocation` (`self.GetTransform`))
  (set `self.LerpBetweenPosition` 0.0)
  ;[1 1 1] Le timer du passage en vue eclatée
  (bind _returnvalue (`KismetSystemLibrary.K2_SetTimerDelegate` (`|CreateDelegate` :!event `GoTo_Timer`) 0.02 true))
  (set `self.GoToTimer_Key` _returnvalue))

(event `/Game/Main/Tipairua/Blueprints/BPI_Vaa.Vaa_ChangeSize`
  (params (Hand1Location :type "Vector Structure") (Hand2Location :type "Vector Structure"))
  ;[1 1 1] Changer la taille
  (if (`self.bIsExploded`)
    (`self.ChangeSize` Hand1Location Hand2Location)
    (else
      (message `/Game/Main/Tipairua/Blueprints/BPI_Vaa.Vaa_ChangeSize` (`self.GetParentActor`) Hand1Location Hand2Location))))

(event `self.ReceiveTick`
  (params (DeltaSeconds :type "Float (single-precision)"))
  (bind (_vvaaoffset_x _vvaaoffset_y) (`KismetMathLibrary.BreakVector` (`self.vVaaOffset`)))
  (bind (_vvaaoffset_x_2 _vvaaoffset_y_2) (`KismetMathLibrary.BreakVector` (`self.vVaaOffset`)))
  (bind _returnvalue (+ (`self.GetInputAxisValue`) _vvaaoffset_x_2))
  (bind _returnvalue_2 (+ _vvaaoffset_y_2 (`self.GetInputAxisValue`)))
  ;[1 1 1] Make that the joystick can bring closer or drive away the vaa
  (if (`self.bIsExploded`)
    (set `self.vVaaOffset` (`KismetMathLibrary.SelectVector` (`KismetMathLibrary.MakeVector` _returnvalue _returnvalue_2) (`KismetMathLibrary.MakeVector` (+ (`self.GetInputAxisValue`) _vvaaoffset_x) (+ _vvaaoffset_y (`self.GetInputAxisValue`))) (or (!= _returnvalue 0.0) (!= _returnvalue_2 0.0))))
    (else
      (`/Engine/EditorBlueprintResources/StandardMacros.DoOnce` false :!via `Reset`
        (:`Completed`
          (set `self.vVaaOffset` (0.0 0.0 0.0)))))))

(event `/Game/Main/Tipairua/Blueprints/BPI_Vaa.Vaa_AttachPiece`
  (params (ControllerToAttached :type "SceneComponent Object Reference"))
  ;[1 1 1] Attacher a la main
  (if (`self.bIsExploded`)
    (`self.K2_AttachToComponent` ControllerToAttached "None" "KeepWorld" "KeepWorld" "KeepWorld")
    (else
      (message `/Game/Main/Tipairua/Blueprints/BPI_Vaa.Vaa_AttachPiece` (`self.GetParentActor`) ControllerToAttached))))

(event `/Game/Main/Tipairua/Blueprints/BPI_Vaa.Vaa_SetDistance`
  (params (Target :type "Vector Structure") (Axis :type "Float (single-precision)"))
  ;[1 1 1] Set Distance qith Joysticks
  (if (`self.bIsExploded`)
    (`self.SetVaaDistance` Target Axis)
    (else
      (message `/Game/Main/Tipairua/Blueprints/BPI_Vaa.Vaa_SetDistance` (`self.GetParentActor`) Target Axis))))

(event `/Game/Main/Tipairua/Blueprints/BPI_Vaa.Vaa_ReleasePiece`
  ;[1 1 1] Detacher a la main
  (if (`self.bIsExploded`)
    (`self.K2_DetachFromActor` "KeepWorld" "KeepWorld" "KeepWorld")
    (else
      (message `/Game/Main/Tipairua/Blueprints/BPI_Vaa.Vaa_ReleasePiece` (`self.GetParentActor`)))))

(event `/Game/Main/Tipairua/Blueprints/BPI_Vaa.PiecesSetIndex`
  (params (Index :type Integer))
  ;[1 1 1] Set l'index de la piece pour la retrouver
  (set `self.Index` Index))

(fn `ChangeSize`
  (params (Hand1Rotation :type "Vector Structure") (Hand2Rotation :type "Vector Structure"))
  (locals (Hand1 :type "Vector Structure") (Hand2 :type "Vector Structure") (NewTrasforms :type "Transform Structure"))
  (bind (_returnvalue_roll _returnvalue_pitch _returnvalue_yaw) (`KismetMathLibrary.BreakRotator` (`KismetMathLibrary.FindLookAtRotation` (`local.Hand1`) (`local.Hand2`))))
  (bind _returnvalue (* (`KismetMathLibrary.VSize` (- (`local.Hand1`) (`local.Hand2`))) 0.001))
  (set `local.Hand1` Hand1Rotation)
  (set `local.Hand2` Hand2Rotation)
  ;[1 1 1] Set le nouveau transform de la pirogue en fonction de la position des mains
  (set `local.NewTrasforms` (`KismetMathLibrary.MakeTransform` (+ (/ (+ (`local.Hand1`) (`local.Hand2`)) 2.0) (`self.vVaaOffset`)) (`KismetMathLibrary.MakeRotator` 0.0 _returnvalue_pitch _returnvalue_yaw) (`KismetMathLibrary.MakeVector` _returnvalue _returnvalue _returnvalue)))
  ;[1 1 1] Verifie si la pirogue est assez proche
  (if (`KismetMathLibrary.NearlyEqual_TransformTransform` (`local.NewTrasforms`) (`self.GetTransform`) 1.0 0.1 0.01)
    ;[1 1 1] Si oui, set direct les nouveaux transforms
    (`self.K2_SetActorTransform` (`local.NewTrasforms`))
    (else
      ;[1 1 1] Sinon, lerp jusqu'a eux
      (`self.K2_SetActorTransform` (`KismetMathLibrary.TLerp` (`self.GetTransform`) (`local.NewTrasforms`) 0.1)))))

(fn `GoTo_Timer`
  ;[1 1 1] Lerp jusqu'a la destination
  (if (`KismetMathLibrary.NearlyEqual_TransformTransform` (`self.Destination`) (`self.GetTransform`) 0.1 0.1 0.1)
    (`KismetSystemLibrary.K2_ClearAndInvalidateTimerHandle` (`self.GoToTimer_Key`))
    (`self.K2_SetActorTransform` (`self.Destination`))
    (else
      (`self.K2_SetActorTransform` (`KismetMathLibrary.TLerp` (`self.OriginalLocation`) (`self.Destination`) (`self.LerpBetweenPosition`)))
      (set `self.LerpBetweenPosition` (+ (`self.LerpBetweenPosition`) 0.04)))))

(fn `SetVaaDistance`
  (params (Target :type "Vector Structure") (Axis :type "Float (double-precision)"))
  ;[1 1 1] Lerp entre la position de la pirogue vers la position de la main
  (`self.K2_SetActorLocation` (`KismetMathLibrary.VLerp` (`self.K2_GetActorLocation`) Target (/ (* Axis -1.0) 30.0))))

(fn `UserConstructionScript`)