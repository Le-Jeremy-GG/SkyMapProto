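; VR-interactable Tipairua double canoe built from child-actor pieces, with a hologram materialize effect on spawn and an exploded view.
; SetPieces indexes the pieces with original and exploded anchor components, which Explode and Gather send to each piece as target transforms.
; While assembled, it can be attached to a controller, pulled along an axis, or smoothly rotated and scaled from two hand positions.
; Materialization drives a material parameter collection and Niagara height from one timeline.
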(event `self.ReceiveBeginPlay`
  (`self.SetPieces`)
  (`KismetSystemLibrary.Delay` 1.0)
  (`self.Vaa_Materialize` true))

(event `self.Vaa_AttachPiece`
  (params (ControllerToAttached :type "SceneComponent Object Reference"))
  ;[1 1 1] Attache une piece si explosé
  (if (not (`self.bIsExploded`))
    (`self.AttachPiece` ControllerToAttached)))

(event `self.Vaa_ReleasePiece`
  ;[1 1 1] Release le vaa
  (if (not (`self.bIsExploded`))
    (`self.K2_DetachFromActor` "KeepWorld" "KeepWorld" "KeepWorld")))

(event `self.Vaa_ReattachPieceToOriginal`
  (params (Index :type Integer))
  ;[1 1 1] Reattach Tipairua qd fini
  (`self.K2_AttachToComponent` (`|GetArrayItem` (`self.ChildrenActors`) Index) (`|GetArrayItem` (`self.ChildrenExplodedPositions`) Index) "None" "KeepWorld" "KeepWorld" "KeepWorld" true))

(event `self.Vaa_ChangeSize`
  (params (Hand1Location :type "Vector Structure") (Hand2Location :type "Vector Structure"))
  ;[1 1 1] Change la taille qd grab avec les deux mains
  (if (not (`self.bIsExploded`))
    (`self.SetVaaSize` Hand1Location Hand2Location)
    (`KismetSystemLibrary.PrintString` "Hello")))

(event `self.Vaa_SetExplodedView`
  (params (Exploded :type Boolean))
  ;[1 1 1] Lance la vue explosee
  (bind _output_get (set `self.bIsExploded` Exploded))
  (if _output_get
    (`self.Explode`)
    (else
      (`self.ReattachAllPieces`)
      (`self.Gather`))))

(event `self.ReceiveTick`
  (params (DeltaSeconds :type "Float (single-precision)"))
  (bind (_vvaaoffset_x _vvaaoffset_y) (`KismetMathLibrary.BreakVector` (`self.vVaaOffset`)))
  (set `self.vVaaOffset` (`KismetMathLibrary.MakeVector` (+ (+ (`self.GetInputAxisValue`) (`self.GetInputAxisValue`)) _vvaaoffset_x) (+ _vvaaoffset_y (+ (`self.GetInputAxisValue`) (`self.GetInputAxisValue`))))))

(event `self.Vaa_SetDistance`
  (params (Target :type "Vector Structure") (Axis :type "Float (single-precision)"))
  (if (not (`self.bIsExploded`))
    (`self.SetVaaDistance` Target Axis)))

(event `self.Vaa_Materialize`
  (params (Appears :type Boolean))
  (bind _holoeffect (`self.HoloEffect`))
  (bind _returnvalue (`NiagaraFunctionLibrary.SpawnSystemAtLocation` "/Game/Main/Tipairua/VFX/NE_TipairuaHoloToBase_System.NE_TipairuaHoloToBase_System" (`self.K2_GetActorLocation`) (`self.K2_GetActorRotation`)))
  (set `self.HoloEffect` _returnvalue)
  (`KismetSystemLibrary.Delay` 0.1)
  (bind (_direction _lerpvalue) (`Timeline|LerpVaa`)
    (:`Update`
      (`KismetMaterialLibrary.SetScalarParameterValue` "/Game/Main/Materials/MPC_Speed.MPC_Speed" "TipairuaHologramHeight" _lerpvalue)
      (`/Engine/EditorBlueprintResources/StandardMacros.IsValid` _holoeffect
        (:`Is Valid`
          (`FXSystemComponent.SetFloatParameter` _holoeffect "MyHeight" (- _lerpvalue 120.0)))))))

(fn `AttachPiece`
  (params (ControllerToAttach :type "SceneComponent Object Reference"))
  (locals (Hand1 :type "Vector Structure") (Hand2 :type "Vector Structure") (NewTrasforms :type "Transform Structure"))
  (`self.K2_AttachToComponent` ControllerToAttach "None" "KeepWorld" "KeepWorld" "KeepWorld")
  (return))

(fn `Explode`
  ;[1 1 1] Initialise l'eclatage en renseignant chaque piece sur sa destination
  (for (_array_element _array_index) (`self.ChildrenActors`)
    (bind _output (`|GetArrayItem` (`self.ChildrenExplodedPositions`) _array_index))
    (message `/Game/Main/Tipairua/Blueprints/BPI_Vaa.Pieces_SetExplodedView` _array_element true (`KismetMathLibrary.MakeTransform` (`SceneComponent.K2_GetComponentLocation` _output) (`SceneComponent.K2_GetComponentRotation` _output) (`SceneComponent.K2_GetComponentScale` _output))))
  (return))

(fn `Gather`
  ;[1 1 1] Annule l'eclatage et renvoie la piece a son point d'origine
  (for (_array_element _array_index) (`self.ChildrenActors`)
    (bind _output (`|GetArrayItem` (`self.ChildrenOriginalPositions`) _array_index))
    (message `/Game/Main/Tipairua/Blueprints/BPI_Vaa.Pieces_SetExplodedView` _array_element false (`KismetMathLibrary.MakeTransform` (`SceneComponent.K2_GetComponentLocation` _output) (`SceneComponent.K2_GetComponentRotation` _output) (`SceneComponent.K2_GetComponentScale` _output))))
  (return))

(fn `ReattachAllPieces`
  (for (_array_element _array_index) (`self.ChildrenActors`)
    (`self.K2_AttachToComponent` _array_element (`|GetArrayItem` (`self.ChildrenOriginalPositions`) _array_index) "None" "KeepWorld" "KeepWorld" "KeepWorld" true)))

(fn `SetPieces`
  ;[1 1 1] Set les arrays contenant les pieces, leurs points d'origine lorsque non éclatées et leurs points d'arrivée lorsque eclatées
  (set `self.ChildrenActors` (`|MakeArray` (`ChildActorComponent.ChildActor` (`self.CanoeL`)) (`ChildActorComponent.ChildActor` (`self.CanoeR`)) (`ChildActorComponent.ChildActor` (`self.Deck`)) (`ChildActorComponent.ChildActor` (`self.Fare`)) (`ChildActorComponent.ChildActor` (`self.HorizontalSticks`)) (`ChildActorComponent.ChildActor` (`self.FrontRopes`)) (`ChildActorComponent.ChildActor` (`self.BackRopes`)) (`ChildActorComponent.ChildActor` (`self.SailSupportFront_1`)) (`ChildActorComponent.ChildActor` (`self.SailSupportFront_2`)) (`ChildActorComponent.ChildActor` (`self.SailFront`)) (`ChildActorComponent.ChildActor` (`self.SailBack`)) (`ChildActorComponent.ChildActor` (`self.SailSupportBack_1`)) (`ChildActorComponent.ChildActor` (`self.SailSupportBack_2`))))
  (set `self.ChildrenOriginalPositions` (`|MakeArray` (`self.OriginalCanoeL`) (`self.OriginalCanoeR`) (`self.OriginalDeck`) (`self.OriginalFare`) (`self.OriginalHorizontalSticks`) (`self.OriginalFrontRopes`) (`self.OriginalBackRopes`) (`self.OriginalSailSupportFront_1`) (`self.OriginalSailSupportFront_2`) (`self.OriginalSailFront`) (`self.OriginalSailBack`) (`self.OriginalSailSupportBack_1`) (`self.OriginalSailSupportBack_2`)))
  (set `self.ChildrenExplodedPositions` (`|MakeArray` (`self.EndCanoeL`) (`self.EndCanoeR`) (`self.EndDeck`) (`self.EndFare`) (`self.EndHorizontalSticks`) (`self.EndFrontRopes`) (`self.EndBackRopes`) (`self.EndSailSupportFront_1`) (`self.EndSailSupportFront_2`) (`self.EndSailFront`) (`self.EndSailBack`) (`self.EndSailSupportBack_1`) (`self.EndSailSupportBack_2`)))
  (for (_array_element _array_index) (`self.ChildrenActors`)
    (message `/Game/Main/Tipairua/Blueprints/BPI_Vaa.PiecesSetIndex` _array_element _array_index))
  (return))

(fn `SetVaaDistance`
  (params (Target :type "Vector Structure") (Axis :type "Float (double-precision)"))
  ;[1 1 1] Lerp entre la position de la pirogue vers la position de la main
  (`self.K2_SetActorLocation` (`KismetMathLibrary.VLerp` (`self.K2_GetActorLocation`) Target (/ (* Axis -1.0) 30.0))))

(fn `SetVaaSize`
  (params (Hand1Rotation :type "Vector Structure") (Hand2Rotation :type "Vector Structure"))
  (locals (Hand1 :type "Vector Structure") (Hand2 :type "Vector Structure") (NewTrasforms :type "Transform Structure"))
  (bind (_returnvalue_roll _returnvalue_pitch _returnvalue_yaw) (`KismetMathLibrary.BreakRotator` (`KismetMathLibrary.FindLookAtRotation` (`local.Hand1`) (`local.Hand2`))))
  (bind _returnvalue (* (`KismetMathLibrary.VSize` (- (`local.Hand1`) (`local.Hand2`))) 0.001))
  (set `local.Hand1` Hand1Rotation)
  (set `local.Hand2` Hand2Rotation)
  ;[1 1 1] Set le nouveau transform de la pirogue en fonction de la position des mains
  (set `local.NewTrasforms` (`KismetMathLibrary.MakeTransform` (`self.K2_GetActorLocation`) (`KismetMathLibrary.MakeRotator` 0.0 _returnvalue_pitch _returnvalue_yaw) (`KismetMathLibrary.MakeVector` _returnvalue _returnvalue _returnvalue)))
  ;[1 1 1] Verifie si la pirogue est assez proche
  (if (`KismetMathLibrary.NearlyEqual_TransformTransform` (`local.NewTrasforms`) (`self.GetTransform`) 1.0 0.1 0.01)
    ;[1 1 1] Si oui, set direct les nouveaux transforms
    (`self.K2_SetActorTransform` (`local.NewTrasforms`))
    (else
      ;[1 1 1] Sinon, lerp jusqu'a eux
      (`self.K2_SetActorTransform` (`KismetMathLibrary.TLerp` (`self.GetTransform`) (`local.NewTrasforms`) 0.1)))))

(fn `SetVaaTransforms`
  (params (Hand1Rotation :type "Vector Structure") (Hand2Rotation :type "Vector Structure"))
  (locals (Hand1 :type "Vector Structure") (Hand2 :type "Vector Structure") (NewTrasforms :type "Transform Structure"))
  (bind (_returnvalue_roll _returnvalue_pitch _returnvalue_yaw) (`KismetMathLibrary.BreakRotator` (`KismetMathLibrary.FindLookAtRotation` (`local.Hand1`) (`local.Hand2`))))
  (bind _returnvalue (* (`KismetMathLibrary.VSize` (- (`local.Hand1`) (`local.Hand2`))) 0.001))
  (set `local.Hand1` Hand1Rotation)
  (set `local.Hand2` Hand2Rotation)
  ;[1 1 1] Set le nouveau transform de la pirogue en fonction de la position des mains
  (set `local.NewTrasforms` (`KismetMathLibrary.MakeTransform` (+ (/ (+ (`local.Hand1`) (`local.Hand2`)) 2.0) (`self.vVaaOffset`)) (`KismetMathLibrary.MakeRotator` 0.0 _returnvalue_pitch _returnvalue_yaw) (`KismetMathLibrary.MakeVector` _returnvalue _returnvalue _returnvalue)))
  ;[1 1 1] Verifie si la pirogue est assez proche
  (if (`KismetMathLibrary.NearlyEqual_TransformTransform` (`local.NewTrasforms`) (`self.GetTransform`) 1.0 0.1 0.01)
    ;[1 1 1] Si oui, set direct les nouveaux transforms
    (`self.K2_SetActorTransform` (`local.NewTrasforms`))
    (else
      ;[1 1 1] Sinon, lerp jusqu'a eux
      (`self.K2_SetActorTransform` (`KismetMathLibrary.TLerp` (`self.GetTransform`) (`local.NewTrasforms`) 0.1)))))

(fn `UserConstructionScript`)