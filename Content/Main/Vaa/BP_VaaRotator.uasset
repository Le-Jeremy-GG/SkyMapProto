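; VR grab handle actor that lets a motion controller rotate the Vaa (pirogue) and adjust its own distance from the hand.
; Attaching to the controller starts a looping timer, apparently driving TurnTimer, which adds the handle's rotation change to the Vaa in world space.
; SetVaaDistance lerps the handle toward a target by an alpha from the negated, scaled axis input.
; Release detaches it without clearing the timer.
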(event `self.ReceiveBeginPlay`)

(event `/Game/Main/Vaa/Blueprints/BPI_Vaa.Vaa_AttachPiece`
  (params (ControllerToAttached :type "SceneComponent Object Reference"))
  (`self.K2_AttachToComponent` ControllerToAttached "None" "KeepWorld" "KeepWorld" "KeepWorld")
  (bind _returnvalue (`KismetSystemLibrary.K2_SetTimerDelegate` (`|CreateDelegate` :!event `TurnTimer`) 0.05 true))
  (set `self.TimerKey` _returnvalue))

(event `/Game/Main/Vaa/Blueprints/BPI_Vaa.Vaa_ReleasePiece`
  (`self.K2_DetachFromActor` "KeepWorld" "KeepWorld" "KeepWorld"))

(event `/Game/Main/Vaa/Blueprints/BPI_Vaa.Vaa_SetDistance`
  (params (Target :type "Vector Structure") (Axis :type "Float (single-precision)"))
  (`self.SetVaaDistance` Target Axis))

(fn `SetVaaDistance`
  (params (Target :type "Vector Structure") (Axis :type "Float (double-precision)"))
  ;[1 1 1] Lerp entre la position de la pirogue vers la position de la main
  (`self.K2_SetActorLocation` (`KismetMathLibrary.VLerp` (`self.K2_GetActorLocation`) Target (/ (* Axis -1.0) 30.0))))

(fn `TurnTimer`
  (`self.K2_AddActorWorldRotation` (`self.Vaa`) (`KismetMathLibrary.NormalizedDeltaRotator` (`self.K2_GetActorRotation`) (`self.PreviousRotation`)) false false)
  (set `self.PreviousRotation` (`self.K2_GetActorRotation`)))

(fn `UserConstructionScript`)