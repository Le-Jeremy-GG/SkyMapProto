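; Wind mast actor that varies its tilt and feather animation with the current month from the Date variable.
; A one-second timer picks a seasonal pitch range, sets the feather material's swing vector and randomly triggers new target angles.
; A faster timer steps pitch toward the target, guarded by IsPlayed, with yaw switching between May–September and other months.
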(event `self.ReceiveBeginPlay`
  (`KismetSystemLibrary.K2_SetTimer` null "MainRotation" 1.0 true)
  (bind _returnvalue (`KismetMaterialLibrary.CreateDynamicMaterialInstance` "/Game/Main/Wind/M_WindFeather.M_WindFeather"))
  (bind _output_get (set `self.FeatherMat` _returnvalue))
  (`PrimitiveComponent.SetMaterial` (`self.StaticMesh`) 0 _output_get))

(fn `ChangeRotation`
  (params (Min :type "Float (double-precision)") (Max :type "Float (double-precision)"))
  ;[1 1 1] détermine de façon aléatoire un angle de rotation
  (if (and (== (`KismetMathLibrary.RandomIntegerInRange` 0 1) 1) (not (`self.IsPlayed`)))
    (set `self.IsPlayed` true)
    (`self.RandomRotation` Min Max)
    (`KismetSystemLibrary.K2_SetTimer` null "GradualRotation" 0.1 true)))

(fn `GradualRotation`
  (bind _returnvalue_roll (`KismetMathLibrary.BreakRotator` (`self.K2_GetActorRotation`)))
  (bind _month (`self.month`))
  (if (`KismetMathLibrary.NearlyEqual_FloatFloat` (`self.ParameterValue`) (`self.ValueToGo`) 0.2)
    ;[1 1 1] arrête le changement de rotation
    (set `self.ParameterValue` (`self.ValueToGo`))
    (set `self.IsPlayed` false)
    (`KismetSystemLibrary.K2_ClearTimer` null "GradualRotation")
    (else
      ;[1 1 1] change la rotation
      (bind _output_get (set `self.ParameterValue` (+ (`self.ParameterValue`) (`KismetMathLibrary.SelectFloat` 0.1 -0.1 (> (`self.ValueToGo`) (`self.ParameterValue`))))))
      (if (and (> _month 4) (< _month 10))
        (`self.K2_SetActorRelativeRotation` (`KismetMathLibrary.MakeRotator` _returnvalue_roll _output_get -45.0))
        (else
          (`self.K2_SetActorRelativeRotation` (`KismetMathLibrary.MakeRotator` _returnvalue_roll _output_get 180.0)))))))

(fn `MainRotation`
  (bind _returnvalue (`KismetMathLibrary.MakeColor` 10.0 0.0 0.0 0.0))
  (bind _feathermat (`self.FeatherMat`))
  (bind _month (`self.month`))
  (bind _month_2 (`self.month`))
  (bind (_currentdate_year _currentdate_month) (`KismetMathLibrary.BreakDateTime` (`/Game/Main/Constellations/Blueprints/BP_TimeManager.CurrentDate` (`self.date`))))
  (set `self.month` _currentdate_month)
  (if (or (and (>= _month 5) (< _month 7)) (and (>= _month_2 8) (< _month_2 10)))
    ;[1 1 1] angle de rotation
    (`self.ChangeRotation` 30.0 60.0)
    ;[1 1 1] axe de l'animation
    (`MaterialInstanceDynamic.SetVectorParameterValue` _feathermat "FeatherSwing" (`KismetMathLibrary.MakeColor` -20.0 20.0 0.0 0.0))
    (else
      ;[1 1 1] si juillet
      (if (== (`self.month`) 7)
        (`self.ChangeRotation` 60.0 90.0)
        (`MaterialInstanceDynamic.SetVectorParameterValue` _feathermat "FeatherSwing" _returnvalue)
        (else
          (`self.ChangeRotation` 10.0 30.0)
          (`MaterialInstanceDynamic.SetVectorParameterValue` _feathermat "FeatherSwing" _returnvalue))))))

(fn `RandomRotation`
  (params (Min :type "Float (double-precision)") (Max :type "Float (double-precision)"))
  ;[1 1 1] choisi un chiffre au hasard avec une valeur minimale et maximale
  (set `self.ValueToGo` (`KismetMathLibrary.RandomFloatInRange` Min Max))
  (return))

(fn `UserConstructionScript`)