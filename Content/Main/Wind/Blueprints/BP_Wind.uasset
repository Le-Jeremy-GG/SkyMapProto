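; BP_Wind drives seasonal wind in the game, setting intensity, direction and sound from the current date.
; One-second timers write date-based values to MPC_Wind and move the sound actor between southeasterly mara'amu and northerly positions.
; Random gusts ramp intensity gradually, also scaling wind and sea volume.
; Tick accumulates a wrapped Offset in MPC_Wind so cloud materials keep their position when wind parameters change.
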(event EventBeginPlay
  ;[1 1 1] lance la fonction permettant de changer la vitesse du vent suivant la date
  (Utilities|Time|SetTimerbyFunctionName 0 "Wind Speed" 1.0 true)
  ;[1 1 1] lance la fonction permettant de changer la direction du vent suivant la date
  (Utilities|Time|SetTimerbyFunctionName 0 "wind orientation" 1.0 true)
  ;[1 1 1] créée une variable vecteur permettant de récupérer la position du vent et de la manipuler
  (Variables|Default|SetWindLoc (Transformation|GetActorLocation (Variables|Default|GetBP_SoundRef)))
  ;[1 1 1] lance la fonction permettant au son du vent de venir de la bonne direction
  (Utilities|Time|SetTimerbyFunctionName 0 "WindLocation" 1.0 true))

(event EventTick
  (params (DeltaSeconds :type Float%20%28single-precision%29))
  ;[1 1 1] Set l'Offset qui permet aux materials (seulement les nuages pr l'instant) de garder leur position qd on change le material parameter
  (bind _returnvalue (Rendering|Material|GetScalarParameterValue "/Game/Main/Wind/MPC_Wind.MPC_Wind" "wind intensity" :!class /Script/Engine.KismetMaterialLibrary))
  (bind _returnvalue_2 (Rendering|Material|GetVectorParameterValue "/Game/Main/Wind/MPC_Wind.MPC_Wind" "wind direction" :!class /Script/Engine.KismetMaterialLibrary))
  (Variables|Default|SetOffsetX (|(((Delta*Direction)+Offset)%1) (|((Intensity/2500)*Delta) (Utilities|Time|GetWorldDeltaSeconds) _returnvalue) (.r _returnvalue_2) (Variables|Default|GetOffsetX)))
  (Variables|Default|SetOffsetY (|(((Delta*Direction)+Offset)%1) (|((Intensity/2500)*Delta) (Utilities|Time|GetWorldDeltaSeconds) _returnvalue) (.g _returnvalue_2) (Variables|Default|GetOffsetY)))
  (Rendering|Material|SetVectorParameterValue "/Game/Main/Wind/MPC_Wind.MPC_Wind" "Offset" (Math|Color|MakeColor (Variables|Default|GetOffsetX) (Variables|Default|GetOffsetY) 0.0) :!class /Script/Engine.KismetMaterialLibrary))

(event Collision|EventActorBeginOverlap
  (params (OtherActor :type Actor%20Object%20Reference)))

(fn ConstructionScript)

(fn WindSpeed
  (bind _testtime (Variables|Default|GetTestTime))
  (bind _currentdate (Variables|/Game/Main/Constellations/Blueprints/BP_TimeManager.BP_TimeManager_C|GetCurrentDate _testtime))
  (LocalVariables|SetMonth (.month _currentdate))
  (LocalVariables|SetDay (.day _currentdate))
  ;[1 1 1] vérifie si le mois se situe entre mai et juillet , ou entre aout et octobre
  (if (or (and (>= (LocalVariables|GetMonth) 5) (< (LocalVariables|GetMonth) 7)) (and (>= (LocalVariables|GetMonth) 8) (< (LocalVariables|GetMonth) 10)))
    ;[1 1 1] si on est dans la 2e moitié de juin
    (if (and (== (LocalVariables|GetMonth) 6) (>= (LocalVariables|GetDay) 15))
      (CallFunction|ChangeWindSpeed 3.0 7.0)
      (else
        ;[1 1 1] si on est dans la 2e moitié de septembre
        (if (and (== (LocalVariables|GetMonth) 9) (>= (LocalVariables|GetDay) 15))
          (CallFunction|ChangeWindSpeed 1.0 3.0)
          (else
            ;[1 1 1] règle la puissance du vent selon le mois
            (bind _output_get (Variables|Default|SetParameter%20Value 3.0))
            (Rendering|Material|SetScalarParameterValue "/Game/Main/Wind/MPC_Wind.MPC_Wind" "wind intensity" _output_get :!class /Script/Engine.KismetMaterialLibrary)
            ;[1 1 1] bourasques
            (CallFunction|ChangeWindSpeed 2.0 3.0)))))
    (else
      ;[1 1 1] vérifie si on est dans la 2e moitié d'avril
      (if (and (== (LocalVariables|GetMonth) 4) (>= (LocalVariables|GetDay) 15))
        ;[1 1 1] gère les bourasques de vent suivant sa puissance
        (CallFunction|ChangeWindSpeed 1.0 3.0)
        (else
          ;[1 1 1] vérifie si on est en juillet
          (if (== (LocalVariables|GetMonth) 7)
            ;[1 1 1] si on est dans la 2e moitié de juillet
            (if (and (== (LocalVariables|GetMonth) 7) (>= (LocalVariables|GetDay) 15))
              (CallFunction|ChangeWindSpeed 4.0 7.0)
              (else
                (bind _output_get_2 (Variables|Default|SetParameter%20Value 5.0))
                (Rendering|Material|SetScalarParameterValue "/Game/Main/Wind/MPC_Wind.MPC_Wind" "wind intensity" _output_get_2 :!class /Script/Engine.KismetMaterialLibrary)
                (CallFunction|ChangeWindSpeed 4.0 5.0)))
            (else
              (bind _output_get_3 (Variables|Default|SetParameter%20Value 1.0))
              (Rendering|Material|SetScalarParameterValue "/Game/Main/Wind/MPC_Wind.MPC_Wind" "wind intensity" _output_get_3 :!class /Script/Engine.KismetMaterialLibrary)
              (CallFunction|ChangeWindSpeed 0.5 1.0))))))))

(fn WindOrientation
  (bind _testtime (Variables|Default|GetTestTime))
  (bind _currentdate (Variables|/Game/Main/Constellations/Blueprints/BP_TimeManager.BP_TimeManager_C|GetCurrentDate _testtime))
  ;[1 1 1] vérifie si on se trouve dans la période déterminée précédemment ,
  (if (and (>= (.month _currentdate) 5) (< (.month _currentdate) 10))
    ;[1 1 1] fait en sorte que le vent vienne du sud-est (mara'amu)
    (Rendering|Material|SetVectorParameterValue "/Game/Main/Wind/MPC_Wind.MPC_Wind" "wind direction" (Math|Color|MakeColor 1.0 1.0 0.0 0.0) :!class /Script/Engine.KismetMaterialLibrary)
    (else
      ;[1 1 1] fait en sorte que le vent vienne du nord
      (Rendering|Material|SetVectorParameterValue "/Game/Main/Wind/MPC_Wind.MPC_Wind" "wind direction" (Math|Color|MakeColor 0.0 -1.0 0.0 0.0) :!class /Script/Engine.KismetMaterialLibrary))))

(fn WindLocation
  (bind _bp_soundref (Variables|Default|GetBP_SoundRef))
  (bind _testtime (Variables|Default|GetTestTime))
  (bind _windloc (Variables|Default|GetWindLoc))
  (bind _currentdate (Variables|/Game/Main/Constellations/Blueprints/BP_TimeManager.BP_TimeManager_C|GetCurrentDate _testtime))
  ;[1 1 1] vérifie si le mois actuel se situe entre mai et octobre
  (if (and (>= (.month _currentdate) 5) (< (.month _currentdate) 10))
    ;[1 1 1] fait en sorte que le son du vent vienne du sud (mara'amu)
    (Transformation|SetActorLocation _bp_soundref (Variables|Default|GetWindLoc) false false)
    (else
      ;[1 1 1] fait en sorte que le son du vent vienne du nord
      (Transformation|SetActorLocation _bp_soundref (Math|Vector|MakeVector (+ (.x _windloc) 4e+03) (- (.y _windloc) 1.8e+03) (.z _windloc)) false false))))

(fn GradualSpeed
  ;[1 1 1] Est-ce quon est assez proche
  (if (Math|Float|NearlyEqual(Float) (Variables|Default|GetParameter%20Value) (Variables|Default|GetValueToGo) 0.2)
    (Variables|Default|SetParameter%20Value (Variables|Default|GetValueToGo))
    (Variables|Default|SetIsAlreadyPlaying false)
    (Utilities|Time|ClearTimerbyFunctionName 0 "GradualSpeed")
    (else
      ;[1 1 1] change la valeur de la puissance du vent si la valeur aléatoire
      (bind _output_get (Variables|Default|SetParameter%20Value (+ (Variables|Default|GetParameter%20Value) (Math|Float|SelectFloat 0.1 -0.1 (> (Variables|Default|GetValueToGo) (Variables|Default|GetParameter%20Value))))))
      (Rendering|Material|SetScalarParameterValue "/Game/Main/Wind/MPC_Wind.MPC_Wind" "wind intensity" _output_get :!class /Script/Engine.KismetMaterialLibrary)
      (Audio|Components|Audio|SetVolumeMultiplier (Variables|/Game/Main/Wind/Blueprints/BP_Sound.BP_Sound_C|GetSeaSound (Variables|Default|GetBP_SoundRef)) (Variables|Default|GetParameter%20Value) :!class /Script/Engine.AudioComponent)
      (Development|PrintString (Utilities|String|Append "ValueTo Go: " (Utilities|String|ToString(Float) (Variables|Default|GetValueToGo)) " 
Actual Value: " (Utilities|String|ToString(Float) (Variables|Default|GetParameter%20Value)))))))

(fn GradualSpeedDown
  (params (NewParameter :type Float%20%28single-precision%29))
  ;[1 1 1] Controle qu'on a pas encore qtteint la valeur du Mara'amu
  (if (> (Variables|Default|GetParameter%20Value) NewParameter)
    (bind _output_get (Variables|Default|SetParameter%20Value (- (Variables|Default|GetParameter%20Value) 0.2)))
    (Rendering|Material|SetScalarParameterValue "/Game/Main/Wind/MPC_Wind.MPC_Wind" "wind intensity" _output_get :!class /Script/Engine.KismetMaterialLibrary)
    (Audio|Components|Audio|SetVolumeMultiplier (Variables|/Game/Main/Wind/Blueprints/BP_Sound.BP_Sound_C|GetSeaSound (Variables|Default|GetBP_SoundRef)) (Variables|Default|GetParameter%20Value) :!class /Script/Engine.AudioComponent)
    (elif (<= (Variables|Default|GetParameter%20Value) NewParameter)
      ;[1 1 1] Sinon arrete la fonction
      (Variables|Default|SetParameter%20Value NewParameter))))

(fn RandomWindSpeed
  (params (Min :type Float%20%28single-precision%29) (Max :type Float%20%28single-precision%29))
  ;[1 1 1] Choisit une valeur aleatoire entre le min et le max et renvoie le resultat au Gradual Speed
  (Variables|Default|SetValueToGo (Math|Random|RandomFloatinRange Min Max))
  (return))

(fn ChangeWindSpeed
  (params (Min :type Float%20%28single-precision%29) (Max :type Float%20%28single-precision%29))
  ;[1 1 1] détermine de façon aléatoire s'il y a des variations de la puissance du vent pour en faire des bourasques
  (if (and (== (Math|Random|RandomIntegerinRange 0 1) 1) (not (Variables|Default|GetIsAlreadyPlaying)))
    (Variables|Default|SetIsAlreadyPlaying true)
    (CallFunction|RandomWindSpeed Min Max)
    (Utilities|Time|SetTimerbyFunctionName 0 "GradualSpeed" 0.1 true)))

(fn FeatherAnim
  (if true
    _))