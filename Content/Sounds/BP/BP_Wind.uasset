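; BP_Wind switches the game's wind between two states, driving both vegetation and sound from the seconds value of TestTime's current date.
; Three looping half-second timers check a five-second threshold.
; They set wind intensity and direction in MPC_vegetation, apply the intensity as SeaSound's volume multiplier on BPSoundRef, and shift that actor between its start and offset location.
; A boolean latch limits intensity and volume writes to state changes; sound-cue swapping is unwired.
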(event `self.ReceiveBeginPlay`
  (`KismetSystemLibrary.K2_SetTimer` null "Wind Speed" 0.5 true)
  (`KismetSystemLibrary.K2_SetTimer` null "wind orientation" 0.5 true)
  (set `self.WindLoc` (`self.K2_GetActorLocation` (`self.BP_SoundRef`)))
  (`KismetSystemLibrary.K2_SetTimer` null "WindLocation" 0.5 true))

(event `self.ReceiveTick`
  (params (DeltaSeconds :type "Float (single-precision)")))

(fn `UserConstructionScript`)

(fn `wind orientation`
  (bind (_currentdate_year _currentdate_month _currentdate_day _currentdate_hour _currentdate_minute _currentdate_second) (`KismetMathLibrary.BreakDateTime` (`/Game/Main/Constellations/Blueprints/BP_TimeManager.CurrentDate` (`self.TestTime`))))
  (if (< _currentdate_second 5)
    (`KismetMaterialLibrary.SetVectorParameterValue` "/Game/MPC_vegetation.MPC_vegetation" "wind direction" (`KismetMathLibrary.MakeColor` 0.0 1.0 0.0 0.0))
    (else
      (`KismetMaterialLibrary.SetVectorParameterValue` "/Game/MPC_vegetation.MPC_vegetation" "wind direction" (`KismetMathLibrary.MakeColor` 0.0 -1.0 0.0 0.0)))))

(fn `Wind Speed`
  (bind _bsuperior5 (`self.bSuperior5`))
  (bind (_currentdate_year _currentdate_month _currentdate_day _currentdate_hour _currentdate_minute _currentdate_second) (`KismetMathLibrary.BreakDateTime` (`/Game/Main/Constellations/Blueprints/BP_TimeManager.CurrentDate` (`self.TestTime`))))
  (if (and (< _currentdate_second 5) _bsuperior5)
    (set `self.bSuperior5` false)
    (bind _output_get (set `self.Parameter Value` 3.0))
    (`KismetMaterialLibrary.SetScalarParameterValue` "/Game/MPC_vegetation.MPC_vegetation" "wind intensity" _output_get)
    ;[1 1 1] change le volume suivant la force du vent
    (`AudioComponent.SetVolumeMultiplier` (`/Game/Sounds/BP/BP_Sound.SeaSound` (`self.BP_SoundRef`)) (`self.Parameter Value`) :!label _label)
    (elif (and (>= _currentdate_second 5) (not _bsuperior5))
      (set `self.bSuperior5` true)
      (bind _output_get_2 (set `self.Parameter Value` 1.0))
      (`KismetMaterialLibrary.SetScalarParameterValue` "/Game/MPC_vegetation.MPC_vegetation" "wind intensity" _output_get_2)
      (goto _label))))

(fn `WindLocation`
  (bind _bp_soundref (`self.BP_SoundRef`))
  (bind (_windloc_x _windloc_y _windloc_z) (`KismetMathLibrary.BreakVector` (`self.WindLoc`)))
  (bind (_currentdate_year _currentdate_month _currentdate_day _currentdate_hour _currentdate_minute _currentdate_second) (`KismetMathLibrary.BreakDateTime` (`/Game/Main/Constellations/Blueprints/BP_TimeManager.CurrentDate` (`self.TestTime`))))
  (if (< _currentdate_second 5)
    (`self.K2_SetActorLocation` _bp_soundref (`KismetMathLibrary.MakeVector` (- _windloc_x 1500.0) _windloc_y _windloc_z) false false)
    (else
      (`self.K2_SetActorLocation` _bp_soundref (`self.WindLoc`) false false))))