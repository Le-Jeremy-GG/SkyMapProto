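; BP_Wind drives wind for both vegetation and audio, switching state based on the current second from TestTime's date.
; BeginPlay starts three half-second looping timers for speed, direction and sound location.
; While the second is under five, wind intensity in MPC_vegetation and BPSon's audio volume rise, direction flips, and BPSon shifts along X.
; Otherwise, intensity, volume and direction switch back and BPSon returns to its starting location.
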(event `self.ReceiveBeginPlay`
  (`KismetSystemLibrary.K2_SetTimer` null "Wind Speed" 0.5 true)
  (`KismetSystemLibrary.K2_SetTimer` null "wind orientation" 0.5 true)
  (set `self.WindLoc` (`self.K2_GetActorLocation` (`self.BP_Son`)))
  (`KismetSystemLibrary.K2_SetTimer` null "WindLocation" 0.5 true))

(event `self.ReceiveTick`
  (params (DeltaSeconds :type "Float (single-precision)")))

(fn `UserConstructionScript`)

(fn `wind orientation`
  (bind (_currentdate_year _currentdate_month _currentdate_day _currentdate_hour _currentdate_minute _currentdate_second) (`KismetMathLibrary.BreakDateTime` (`/Game/Main/Constellations/Blueprints/BP_TimeManager.CurrentDate` (`self.TestTime`))))
  (if (< _currentdate_second 5)
    (`KismetMaterialLibrary.SetVectorParameterValue` "/Game/MPC_vegetation.MPC_vegetation" "wind direction" (`KismetMathLibrary.MakeColor` 0.0 1.0 0.0 0.0))
    (set `self.Volume Multiplier` (`self.Volume Multiplier`))
    (else
      (`KismetMaterialLibrary.SetVectorParameterValue` "/Game/MPC_vegetation.MPC_vegetation" "wind direction" (`KismetMathLibrary.MakeColor` 0.0 -1.0 0.0 0.0))
      (set `self.Volume Multiplier` 0.5))))

(fn `Wind Speed`
  (bind (_currentdate_year _currentdate_month _currentdate_day _currentdate_hour _currentdate_minute _currentdate_second) (`KismetMathLibrary.BreakDateTime` (`/Game/Main/Constellations/Blueprints/BP_TimeManager.CurrentDate` (`self.TestTime`))))
  (if (< _currentdate_second 5)
    (bind _output_get (set `self.Parameter Value` 3.0))
    (`KismetMaterialLibrary.SetScalarParameterValue` "/Game/MPC_vegetation.MPC_vegetation" "wind intensity" _output_get)
    (else
      (bind _output_get_2 (set `self.Parameter Value` 1.0))
      (`KismetMaterialLibrary.SetScalarParameterValue` "/Game/MPC_vegetation.MPC_vegetation" "wind intensity" _output_get_2)))
  (`AudioComponent.SetVolumeMultiplier` (`/Game/Sounds/BPSon2.AudioWind` (`self.BP_Son`)) (`self.Parameter Value`)))

(fn `WindLocation`
  (bind _bp_son (`self.BP_Son`))
  (bind (_windloc_x _windloc_y _windloc_z) (`KismetMathLibrary.BreakVector` (`self.WindLoc`)))
  (bind (_currentdate_year _currentdate_month _currentdate_day _currentdate_hour _currentdate_minute _currentdate_second) (`KismetMathLibrary.BreakDateTime` (`/Game/Main/Constellations/Blueprints/BP_TimeManager.CurrentDate` (`self.TestTime`))))
  (if (< _currentdate_second 5)
    (`self.K2_SetActorLocation` _bp_son (`KismetMathLibrary.MakeVector` (- _windloc_x 1500.0) _windloc_y _windloc_z) false false)
    (else
      (`self.K2_SetActorLocation` _bp_son (`self.WindLoc`) false false))))